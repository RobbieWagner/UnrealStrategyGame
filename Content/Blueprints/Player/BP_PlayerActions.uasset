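; Player input actor for a tile grid that tracks the hovered and selected tiles and units and runs swappable mouse actions.
; Each tick it resolves the tile and unit under the cursor, preferring unit hits, and updates hover states.
; SetActions spawns action actors for left and right click, executed on press and on hover changes while held, enabling drag.
; Selections toggle tile and unit states, responding to grid regeneration and tile updates.
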(event Custom|OnHoverTileChanged
  (Utilities|FlowControl|Sequence
    (:then_0
      (if (Variables|Default|GetIsLMBDown)
        (Utilities|IsValid (Variables|Default|GetLeftClickAction)
          (:Is%20Valid
            (Default|ExecuteAction (Variables|Default|GetLeftClickAction) (Variables|Default|GetHoveredTile))))))
    (:then_1
      (if (Variables|Default|GetIsRMBDown)
        (Utilities|IsValid (Variables|Default|GetRightClickAction)
          (:Is%20Valid
            (Default|ExecuteAction (Variables|Default|GetRightClickAction) (Variables|Default|GetHoveredTile))))))))

(event EventBeginPlay
  (bind _returnvalue (Actor|GetActorOfClass "/Game/Blueprints/Grid/BP_Grid.BP_Grid_C"))
  (bind _output_get (Variables|Default|SetGrid _returnvalue))
  (EventDispatchers|BindEventtoOnGridGenerated _output_get (EventDispatchers|CreateEvent :!event OnGridGenerated))
  (EventDispatchers|BindEventtoOnTileDataUpdated _output_get (EventDispatchers|CreateEvent :!event OnTileDataUpdated))
  (bind _returnvalue_2 (Actor|GetActorOfClass "/Game/Combat/BP_CombatManager.BP_CombatManager_C"))
  (Variables|Default|SetCombatManager _returnvalue_2)
  (Input|EnableInput (Game|GetPlayerController 0)))

(event EventTick
  (params (DeltaSeconds :type Float%20%28single-precision%29))
  (CallFunction|UpdateTileandUnitUnderCursor))

(event Input|MouseEvents|LeftMouseButton
  (params (Key :type Key%20Structure))
  (:Pressed
    (CallFunction|UpdateTileandUnitUnderCursor)
    (Variables|Default|SetIsLMBDown true)
    (Utilities|IsValid (Variables|Default|GetLeftClickAction)
      (:Is%20Valid
        (Default|ExecuteAction (Variables|Default|GetLeftClickAction) (Variables|Default|GetHoveredTile)))))
  (:Released
    (Variables|Default|SetIsLMBDown false)))

(event Input|MouseEvents|RightMouseButton
  (params (Key :type Key%20Structure))
  (:Pressed
    (CallFunction|UpdateTileandUnitUnderCursor)
    (Variables|Default|SetIsRMBDown true)
    (Utilities|IsValid (Variables|Default|GetRightClickAction)
      (:Is%20Valid
        (Default|ExecuteAction (Variables|Default|GetRightClickAction) (Variables|Default|GetHoveredTile)))))
  (:Released
    (Variables|Default|SetIsRMBDown false)))

(fn ConstructionScript)

(fn UpdateTileandUnitUnderCursor
  (Utilities|FlowControl|Sequence
    (:then_0
      (bind _unit (CallFunction|GetUnitUnderCursor))
      (if (!= _unit (Variables|Default|GetHoveredUnit))
        (Utilities|FlowControl|Sequence
          (:then_0
            (Utilities|IsValid (Variables|Default|GetHoveredUnit)
              (:Is%20Valid
                (Default|RemoveStatefromUnit (Variables|Default|GetHoveredUnit) "NewEnumerator1")
                (Variables|Default|SetHoveredUnit 0))))
          (:then_1
            (Utilities|IsValid _unit
              (:Is%20Valid
                (bind _output_get (Variables|Default|SetHoveredUnit _unit))
                (Default|AddStatetoUnit _output_get "NewEnumerator1")
                (LocalVariables|SetHoveredUnitIndex (Variables|/Game/Blueprints/Units/BP_Unit.BP_Unit_C|GetCurrentGridIndex _output_get))))))
        (else
          (Utilities|IsValid _unit
            (:Is%20Valid
              (LocalVariables|SetHoveredUnitIndex (Variables|/Game/Blueprints/Units/BP_Unit.BP_Unit_C|GetCurrentGridIndex _unit)))))))
    (:then_1
      (Utilities|IsValid (Variables|Default|GetHoveredUnit)
        (:Is%20Valid
          (if (!= (LocalVariables|GetHoveredUnitIndex) (Variables|Default|GetHoveredTile))
            (Default|RemoveTileStatefromTile (Variables|Default|GetGrid) (Variables|Default|GetHoveredTile) "NewEnumerator1")
            (bind _output_get_2 (Variables|Default|SetHoveredTile (LocalVariables|GetHoveredUnitIndex)))
            (Default|AddTileStatetoTile (Variables|Default|GetGrid) _output_get_2 "NewEnumerator1")
            (CallFunction|OnHoverTileChanged)))
        (:Is%20Not%20Valid
          (bind _index (Default|GetIndexUnderCursor (Variables|Default|GetGrid)))
          (if (!= _index (Variables|Default|GetHoveredTile))
            (Default|RemoveTileStatefromTile (Variables|Default|GetGrid) (Variables|Default|GetHoveredTile) "NewEnumerator1")
            (bind _output_get_3 (Variables|Default|SetHoveredTile _index))
            (Default|AddTileStatetoTile (Variables|Default|GetGrid) _output_get_3 "NewEnumerator1")
            (CallFunction|OnHoverTileChanged)))))))

(fn SetActions
  (params (LeftMouseAction :type BP%20Action%20Class%20Reference) (RightMouseAction :type BP%20Action%20Class%20Reference))
  (Utilities|FlowControl|Sequence
    (:then_0
      (Utilities|IsValid (Variables|Default|GetLeftClickAction)
        (:Is%20Valid
          (Actor|DestroyActor (Variables|Default|GetLeftClickAction))
          (Variables|Default|SetLeftClickAction 0))
        (:Is%20Not%20Valid
          _))
      (if (Utilities|IsValidClass LeftMouseAction)
        (bind _returnvalue (Game|SpawnActorfromClass LeftMouseAction (Math|Transform|MakeTransform "0, 0, 0" "0, 0, 0" "1.000000,1.000000,1.000000") "Undefined" "MultiplyWithRoot" 0 self 0))
        (Variables|Default|SetLeftClickAction _returnvalue)))
    (:then_1
      (Utilities|IsValid (Variables|Default|GetRightClickAction)
        (:Is%20Valid
          (Actor|DestroyActor (Variables|Default|GetRightClickAction))
          (Variables|Default|SetRightClickAction 0))
        (:Is%20Not%20Valid
          _))
      (if (Utilities|IsValidClass RightMouseAction)
        (bind _returnvalue_2 (Game|SpawnActorfromClass RightMouseAction (Math|Transform|MakeTransform "0, 0, 0" "0, 0, 0" "1.000000,1.000000,1.000000") "Undefined" "MultiplyWithRoot" 0 self 0))
        (Variables|Default|SetRightClickAction _returnvalue_2)))
    (:then_2
      (Default|CallOnSelectedActionsChanged (Variables|Default|GetLeftClickAction) (Variables|Default|GetRightClickAction)))))

(fn GetUnitUnderCursor
  (params (PlayerIndex :type Integer))
  (bind _returnvalue (Game|GetPlayerController PlayerIndex))
  (bind (_hitresult _returnvalue_2) (Game|Player|GetHitResultUnderCursorbyChannel _returnvalue "TraceTypeQuery5" false))
  (if _returnvalue_2
    (return (.AsBP%20Unit (Utilities|Casting|CastToBP_Unit (.HitActor (Collision|BreakHitResult _hitresult)))))
    (else
      (bind _index (Default|GetIndexUnderCursor (Variables|Default|GetGrid) PlayerIndex))
      (return (.UnitOnTile (Utilities|Struct|BreakS_TileData (.Value (Utilities|Map|Find (Variables|/Game/Blueprints/Grid/BP_Grid.BP_Grid_C|GetGridTiles (Variables|Default|GetGrid)) _index))))))))

(fn UpdateSelectedTilesandUnits
  (params (Index :type Int%20Point%20Structure) (ForceSelect :type Boolean))
  (Utilities|FlowControl|Sequence
    (:then_0
      (if (or (not (Utilities|Array|ContainsItem (Variables|Default|GetSelectedTiles) Index)) ForceSelect)
        (Default|AddTileStatetoTile (Variables|Default|GetGrid) Index "NewEnumerator2")
        (Utilities|Array|AddUnique (Variables|Default|GetSelectedTiles) Index)
        (else
          (CallFunction|RemoveTilefromSelection Index))))
    (:then_1
      (bind _output_get (LocalVariables|SetUnitOnSelectedTile (.UnitOnTile (Utilities|Struct|BreakS_TileData (.Value (Utilities|Map|Find (Variables|/Game/Blueprints/Grid/BP_Grid.BP_Grid_C|GetGridTiles (Variables|Default|GetGrid)) Index))))))
      (Utilities|IsValid _output_get
        (:Is%20Valid
          (if (or (not (Utilities|Array|ContainsItem (Variables|Default|GetSelectedUnits) (LocalVariables|GetUnitOnSelectedTile))) ForceSelect)
            (if (CallFunction|CanSelectUnit (LocalVariables|GetUnitOnSelectedTile))
              (Default|AddStatetoUnit (LocalVariables|GetUnitOnSelectedTile) "NewEnumerator2")
              (Utilities|Array|AddUnique (Variables|Default|GetSelectedUnits) (LocalVariables|GetUnitOnSelectedTile)))
            (else
              (CallFunction|RemoveUnitfromSelection Index))))))))

(fn CanSelectUnit
  (params (Unit :type BP%20Unit%20Object%20Reference))
  (return true))

(fn ClearAllSelections
  (bind _output_get (LocalVariables|SetCopySelectedTiles (Variables|Default|GetSelectedTiles)))
  (for _array_element _output_get
    (CallFunction|RemoveTilefromSelection _array_element)
    (CallFunction|RemoveUnitfromSelection _array_element))
  (Utilities|Array|Clear (Variables|Default|GetSelectedTiles))
  (Utilities|Array|Clear (Variables|Default|GetSelectedUnits)))

(fn OnGridGenerated
  (CallFunction|ClearAllSelections))

(fn OnTileDataUpdated
  (params (Index :type Int%20Point%20Structure))
  (if (Utilities|Array|ContainsItem (Variables|Default|GetSelectedTiles) Index)
    (if (Default|IsIndexValid (Variables|Default|GetGrid) Index)
      (CallFunction|UpdateSelectedTilesandUnits Index true)
      (else
        (CallFunction|RemoveUnitfromSelection Index)))))

(fn RemoveUnitfromSelection
  (params (Index :type Int%20Point%20Structure))
  (bind _grid (Variables|Default|GetGrid))
  (bind _gridtiles (Variables|/Game/Blueprints/Grid/BP_Grid.BP_Grid_C|GetGridTiles _grid))
  (bind _value (Utilities|Map|Find _gridtiles Index))
  (bind _unitontile (Utilities|Struct|BreakS_TileData _value))
  (Utilities|IsValid _unitontile
    (:Is%20Valid
      (Default|RemoveStatefromUnit _unitontile "NewEnumerator2")
      (Utilities|Array|RemoveItem (Variables|Default|GetSelectedUnits) _unitontile))))

(fn RemoveTilefromSelection
  (params (Index :type Int%20Point%20Structure))
  (Default|RemoveTileStatefromTile (Variables|Default|GetGrid) Index "NewEnumerator2")
  (Utilities|Array|RemoveItem (Variables|Default|GetSelectedTiles) Index))

(fn GetFirstMovableSelectedUnit
  (for _array_element (Variables|Default|GetSelectedUnits)
    (if (Default|CanbeMovedbyPlayer _array_element)
      (return _array_element)))
  (return 0))