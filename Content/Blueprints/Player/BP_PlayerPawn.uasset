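; BP_PlayerPawn is the player pawn that provides a movable, rotatable, zoomable spring arm camera driven by Enhanced Input values.
; Each Tick eases zoom and yaw rates toward input with Lerp, changing the clamped arm length and rotating the SpringArm for smooth acceleration and stopping.
; Panning uses AddMovementInput along the camera's right vector and its up vector projected onto the horizontal plane, keeping movement relative to the view.
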(event Custom|UpdateSmoothZoom
  (bind _springarm (Variables|Default|GetSpringArm))
  (bind _output_get (Variables|Default|SetZoom_Rate (Math|Float|Lerp (Variables|Default|GetZoom_Rate) (* (Input|EnhancedActionValues|GetIA_Zoom) (* (Variables|Default|GetZOOM_INITIAL_SPEED) -1.0)) (* (Utilities|Time|GetWorldDeltaSeconds) 5.0))))
  (Variables|/Script/Engine.SpringArmComponent|SetTargetArmLength _springarm (Math|Float|Clamp(Float) (+ _output_get (Variables|/Script/Engine.SpringArmComponent|GetTargetArmLength _springarm)) (Variables|Default|GetZoomMin) (Variables|Default|GetZoomMax))))

(event Custom|UpdateSmoothRotation
  (bind _output_get (Variables|Default|SetRotation_Rate (Math|Float|Lerp (Variables|Default|GetRotation_Rate) (* (Input|EnhancedActionValues|GetIA_RotateCamera) (Variables|Default|GetROTATION_INITIAL_SPEED)) (* (Utilities|Time|GetWorldDeltaSeconds) 1.9))))
  (Transformation|AddRelativeRotation (Variables|Default|GetSpringArm) (Math|Rotator|MakeRotator 0.0 0.0 _output_get) false false))

(event Custom|UpdateCameraPosition
  (bind _returnvalue (Input|EnhancedActionValues|GetIA_MoveCamera))
  (bind _camera_move_initial_speed (Variables|Default|GetCAMERA_MOVE_INITIAL_SPEED))
  (Pawn|Input|AddMovementInput (Math|Vector|GetRightVector (Variables|Default|GetCamera)) (* (.x _returnvalue) _camera_move_initial_speed) false)
  (Pawn|Input|AddMovementInput (Math|Vector|ProjectVectorontoPlane (Math|Vector|GetUpVector (Variables|Default|GetCamera)) "0.000000,0.000000,1.000000") (* _camera_move_initial_speed (.y _returnvalue)) false))

(event EventBeginPlay)

(event Collision|EventActorBeginOverlap
  (params (OtherActor :type Actor%20Object%20Reference)))

(event EventTick
  (params (DeltaSeconds :type Float%20%28single-precision%29))
  (CallFunction|UpdateSmoothZoom)
  (CallFunction|UpdateSmoothRotation)
  (CallFunction|UpdateCameraPosition))

(fn ConstructionScript)