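; Player action for tactical grid combat that previews a chosen combat action's range and area of effect, then executes it on a target tile.
; Setting the action loads its execution data and marks range tiles from the selected tile through the CombatManager.
; Hovering updates the area overlay around the hovered in-range tile, or around the selected tile for certain source-location types.
; Executing passes origin and target to the CombatManager and deselects the action button; EndPlay clears both overlays.
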(event EventBeginPlay
  (|CallParentFunction) ; This node is disabled and will not be called.\nDrag off pins to build functionality.
)

(event Collision|EventActorBeginOverlap
  (params (OtherActor :type Actor%20Object%20Reference))
  (|CallParentFunction OtherActor) ; This node is disabled and will not be called.\nDrag off pins to build functionality.
)

(event EventTick
  (params (DeltaSeconds :type Float%20%28single-precision%29))
  (|CallParentFunction DeltaSeconds) ; This node is disabled and will not be called.\nDrag off pins to build functionality.
)

(event EventEndPlay
  (params (EndPlayReason :type EEndPlayReason%20Enum :default "Destroyed"))
  (bind _playeractions (Variables|Default|GetPlayerActions))
  (bind _grid (Variables|/Game/Blueprints/Player/BP_PlayerActions.BP_PlayerActions_C|GetGrid _playeractions))
  (|CallParentFunction EndPlayReason)
  (Default|ClearStatefromTiles _grid "NewEnumerator9")
  (Default|ClearStatefromTiles _grid "NewEnumerator8"))

(fn ConstructionScript
  (|CallParentFunction))

(fn SetCombatAction
  (params (Action :type E_CombatAction%20Enum :default "NewEnumerator0"))
  (bind _playeractions (Variables|Default|GetPlayerActions))
  (bind _grid (Variables|/Game/Blueprints/Player/BP_PlayerActions.BP_PlayerActions_C|GetGrid _playeractions))
  (bind _output_get (Variables|Default|SetAction Action))
  (if (Utilities|Enum|NotEqual(Enum) _output_get "NewEnumerator0")
    (bind _data (CallFunction|GetDatafromCombatAction (Variables|Default|GetAction)))
    (Variables|Default|SetExecution (.Execution (Utilities|Struct|BreakS_CombatActionData _data)))
    (Variables|Default|SetExecutionAoE (.AoE (Utilities|Struct|BreakS_CombatActionData _data)))
    (CallFunction|ShowActionRangePattern)
    (else
      (Default|ClearStatefromTiles _grid "NewEnumerator9")
      (Default|ClearStatefromTiles _grid "NewEnumerator8"))))

(fn ShowActionRangePattern
  (bind _playeractions (Variables|Default|GetPlayerActions))
  (bind _playeractions_2 (Variables|Default|GetPlayerActions))
  (bind _grid (Variables|/Game/Blueprints/Player/BP_PlayerActions.BP_PlayerActions_C|GetGrid _playeractions_2))
  (Default|ClearStatefromTiles _grid "NewEnumerator8")
  (Default|ClearStatefromTiles _grid "NewEnumerator9")
  (if (Default|HasSelectedTiles _playeractions)
    (for _array_element (Default|GetActionRange (Variables|/Game/Blueprints/Player/BP_PlayerActions.BP_PlayerActions_C|GetCombatManager _playeractions) (Utilities|Array|Get(acopy) (Variables|/Game/Blueprints/Player/BP_PlayerActions.BP_PlayerActions_C|GetSelectedTiles _playeractions)) (Variables|Default|GetExecution))
      (Default|AddTileStatetoTile (Variables|/Game/Blueprints/Player/BP_PlayerActions.BP_PlayerActions_C|GetGrid (Variables|Default|GetPlayerActions)) _array_element "NewEnumerator8")
      (CallFunction|ShowAOE))))

(fn ExecuteAction
  (params (Index :type Int%20Point%20Structure))
  (bind _playeractions (Variables|Default|GetPlayerActions))
  (bind _playeractions_2 (Variables|Default|GetPlayerActions))
  (|CallParentFunction Index)
  (if (and (Default|HasSelectedTiles _playeractions_2) (Default|HasSelectedUnits _playeractions_2))
    (Default|ExecuteCombatAction (Variables|/Game/Blueprints/Player/BP_PlayerActions.BP_PlayerActions_C|GetCombatManager _playeractions) (Variables|Default|GetAction) (Utilities|Array|Get(acopy) (Variables|/Game/Blueprints/Player/BP_PlayerActions.BP_PlayerActions_C|GetSelectedTiles _playeractions)) Index)
    (Default|SetSelectedActionfromIndex (Variables|/Game/Combat/Widgets/W_Combat.W_Combat_C|GetButtonList_Action (Variables|/Game/Blueprints/Player/BP_PlayerActions.BP_PlayerActions_C|GetW_Combat (Variables|Default|GetPlayerActions))) -1)))

(fn ShowAOE
  (bind _playeractions (Variables|Default|GetPlayerActions))
  (bind _playeractions_2 (Variables|Default|GetPlayerActions))
  (bind _playeractions_3 (Variables|Default|GetPlayerActions))
  (Default|ClearStatefromTiles (Variables|/Game/Blueprints/Player/BP_PlayerActions.BP_PlayerActions_C|GetGrid (Variables|Default|GetPlayerActions)) "NewEnumerator9")
  (if (Utilities|Array|ContainsItem (Utilities|Struct|BreakS_IntPointArray (.Value (Utilities|Map|Find (Variables|/Game/Blueprints/Grid/BP_Grid.BP_Grid_C|GetTilesWithState (Variables|/Game/Blueprints/Player/BP_PlayerActions.BP_PlayerActions_C|GetGrid (Variables|Default|GetPlayerActions))) "NewEnumerator8"))) (Variables|/Game/Blueprints/Player/BP_PlayerActions.BP_PlayerActions_C|GetHoveredTile (Variables|Default|GetPlayerActions)))
    (if (Utilities|Enum|NotEqual(Enum) (.RangePattern (Utilities|Struct|BreakS_CombatAction_Execution (Variables|Default|GetExecutionAoE))) "NewEnumerator0")
      (for _array_element (Default|GetActionRange (Variables|/Game/Blueprints/Player/BP_PlayerActions.BP_PlayerActions_C|GetCombatManager _playeractions) (Variables|/Game/Blueprints/Player/BP_PlayerActions.BP_PlayerActions_C|GetHoveredTile _playeractions) (Variables|Default|GetExecutionAoE))
        (Default|AddTileStatetoTile (Variables|/Game/Blueprints/Player/BP_PlayerActions.BP_PlayerActions_C|GetGrid (Variables|Default|GetPlayerActions)) _array_element "NewEnumerator9"))
      (else
        (Default|AddTileStatetoTile (Variables|/Game/Blueprints/Player/BP_PlayerActions.BP_PlayerActions_C|GetGrid _playeractions_2) (Variables|/Game/Blueprints/Player/BP_PlayerActions.BP_PlayerActions_C|GetHoveredTile _playeractions_2) "NewEnumerator9")))
    (else
      (bind _data (CallFunction|GetDatafromCombatAction (Variables|Default|GetAction)))
      (if (Utilities|Enum|Equal(Enum) (.SourceLocation (Utilities|Struct|BreakS_CombatActionData _data)) "NewEnumerator1")
        (if (and (Utilities|Enum|NotEqual(Enum) (.RangePattern (Utilities|Struct|BreakS_CombatAction_Execution (Variables|Default|GetExecutionAoE))) "NewEnumerator0") (> (Utilities|Array|Length (Variables|/Game/Blueprints/Player/BP_PlayerActions.BP_PlayerActions_C|GetSelectedTiles (Variables|Default|GetPlayerActions))) 0))
          (for _array_element_2 (Default|GetActionRange (Variables|/Game/Blueprints/Player/BP_PlayerActions.BP_PlayerActions_C|GetCombatManager _playeractions_3) (Utilities|Array|Get(acopy) (Variables|/Game/Blueprints/Player/BP_PlayerActions.BP_PlayerActions_C|GetSelectedTiles _playeractions_3)) (Variables|Default|GetExecutionAoE))
            (Default|AddTileStatetoTile (Variables|/Game/Blueprints/Player/BP_PlayerActions.BP_PlayerActions_C|GetGrid (Variables|Default|GetPlayerActions)) _array_element_2 "NewEnumerator9")))))))

(fn ExecuteHoveredAction
  (params (Index :type Int%20Point%20Structure))
  (|CallParentFunction Index)
  (CallFunction|ShowAOE))