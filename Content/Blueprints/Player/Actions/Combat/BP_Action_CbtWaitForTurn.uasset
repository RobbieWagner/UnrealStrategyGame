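; Combat player action, named for waiting for a turn, that previews on the grid where a unit can move.
; On hover it picks the hovered unit, falling back to the first selected one, and re-runs only when that unit changes.
; The grid's reachable pathfinder searches with the unit's movement stats and an off-grid dummy target.
; Returned tiles get a highlight state, cleared before each new search; EndPlay clears a different state.
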(event EventBeginPlay
  (|CallParentFunction)
  (EventDispatchers|BindEventtoOnPathfindingCompleted (Variables|/Game/Blueprints/Grid/BP_Grid.BP_Grid_C|GetGridPathfinding_Reachable (Variables|/Game/Blueprints/Player/BP_PlayerActions.BP_PlayerActions_C|GetGrid (Variables|Default|GetPlayerActions))) (EventDispatchers|CreateEvent :!event OnPathfindingCompleteReachables)))

(event EventEndPlay
  (params (EndPlayReason :type EEndPlayReason%20Enum :default "Destroyed"))
  (|CallParentFunction EndPlayReason)
  (Default|ClearStatefromTiles (Variables|/Game/Blueprints/Player/BP_PlayerActions.BP_PlayerActions_C|GetGrid (Variables|Default|GetPlayerActions)) "NewEnumerator3"))

(fn ConstructionScript
  (|CallParentFunction))

(fn FindReachableTiles
  (params (Unit :type BP%20Unit%20Object%20Reference))
  (if (!= Unit (Variables|Default|GetCurrentUnitForReachables))
    (bind _output_get (Variables|Default|SetCurrentUnitForReachables Unit))
    (Default|ClearStatefromTiles (Variables|/Game/Blueprints/Player/BP_PlayerActions.BP_PlayerActions_C|GetGrid (Variables|Default|GetPlayerActions)) "NewEnumerator4")
    (EventDispatchers|BindEventtoOnPathfindingCompleted (Variables|/Game/Blueprints/Grid/BP_Grid.BP_Grid_C|GetGridPathfinding_Reachable (Variables|/Game/Blueprints/Player/BP_PlayerActions.BP_PlayerActions_C|GetGrid (Variables|Default|GetPlayerActions))) (EventDispatchers|CreateEvent :!event OnPathfindingCompleteReachables))
    (Utilities|IsValid (Variables|Default|GetCurrentUnitForReachables)
      (:Is%20Valid
        (Default|FindPath (Variables|/Game/Blueprints/Grid/BP_Grid.BP_Grid_C|GetGridPathfinding_Reachable (Variables|/Game/Blueprints/Player/BP_PlayerActions.BP_PlayerActions_C|GetGrid (Variables|Default|GetPlayerActions))) (Variables|/Game/Blueprints/Units/BP_Unit.BP_Unit_C|GetCurrentGridIndex _output_get) (Utilities|Struct|MakeIntPoint -999 -999) (.CanWalkDiagonally (Utilities|Struct|BreakS_UnitData_Stats (.Stats (Utilities|Struct|BreakS_UnitData (Variables|/Game/Blueprints/Units/BP_Unit.BP_Unit_C|GetUnitData (Variables|Default|GetCurrentUnitForReachables)))))) (.ValidTileTypes (Utilities|Struct|BreakS_UnitData_Stats (.Stats (Utilities|Struct|BreakS_UnitData (Variables|/Game/Blueprints/Units/BP_Unit.BP_Unit_C|GetUnitData (Variables|Default|GetCurrentUnitForReachables)))))) 0.0 0.0 true (.MoveDistance (Utilities|Struct|BreakS_UnitData_Stats (.Stats (Utilities|Struct|BreakS_UnitData (Variables|/Game/Blueprints/Units/BP_Unit.BP_Unit_C|GetUnitData (Variables|Default|GetCurrentUnitForReachables)))))))))))

(fn OnPathfindingCompleteReachables
  (params (Reachable%20Tiles :type Array%20of%20Int%20Point%20Structures))
  (for _array_element Reachable%20Tiles
    (Default|AddTileStatetoTile (Variables|/Game/Blueprints/Player/BP_PlayerActions.BP_PlayerActions_C|GetGrid (Variables|Default|GetPlayerActions)) _array_element "NewEnumerator4")))

(fn ExecuteHoveredAction
  (params (Index :type Int%20Point%20Structure))
  (bind _playeractions (Variables|Default|GetPlayerActions))
  (bind _hoveredunit (Variables|/Game/Blueprints/Player/BP_PlayerActions.BP_PlayerActions_C|GetHoveredUnit _playeractions))
  (|CallParentFunction Index)
  (Utilities|IsValid _hoveredunit
    (:Is%20Valid
      (CallFunction|FindReachableTiles _hoveredunit))
    (:Is%20Not%20Valid
      (if (> (Utilities|Array|Length (Variables|/Game/Blueprints/Player/BP_PlayerActions.BP_PlayerActions_C|GetSelectedUnits _playeractions)) 0)
        (CallFunction|FindReachableTiles (Utilities|Array|Get(acopy) (Variables|/Game/Blueprints/Player/BP_PlayerActions.BP_PlayerActions_C|GetSelectedUnits (Variables|Default|GetPlayerActions))))))))