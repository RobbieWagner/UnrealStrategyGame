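; Combat move action for the player: previews movement on the grid and moves the selected unit.
; Two grid pathfinders asynchronously mark tiles via completion events: reachable tiles for the hovered or selected unit, and the selected unit's path to the hovered tile.
; Executing passes the cached path to CombatManager.MoveUnit.
; Unit move events clear highlights, block previews during travel, then disable further movement and reselect the unit if it can still act.
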(event EventBeginPlay
  (|CallParentFunction)
  (EventDispatchers|BindEventtoOnPathfindingCompleted (Variables|/Game/Blueprints/Grid/BP_Grid.BP_Grid_C|GetGridPathfinding_Reachable (Variables|/Game/Blueprints/Player/BP_PlayerActions.BP_PlayerActions_C|GetGrid (Variables|Default|GetPlayerActions))) (EventDispatchers|CreateEvent :!event OnPathfindingCompleteReachables))
  (EventDispatchers|BindEventtoOnPathfindingCompleted (Variables|/Game/Blueprints/Grid/BP_Grid.BP_Grid_C|GetGrid%20Pathfinding (Variables|/Game/Blueprints/Player/BP_PlayerActions.BP_PlayerActions_C|GetGrid (Variables|Default|GetPlayerActions))) (EventDispatchers|CreateEvent :!event OnPathFindingCompletedPath))
  (if (> (Utilities|Array|Length (Variables|/Game/Blueprints/Player/BP_PlayerActions.BP_PlayerActions_C|GetSelectedUnits (Variables|Default|GetPlayerActions))) 0)
    (CallFunction|FindReachableTiles (Utilities|Array|Get(acopy) (Variables|/Game/Blueprints/Player/BP_PlayerActions.BP_PlayerActions_C|GetSelectedUnits (Variables|Default|GetPlayerActions))))))

(event EventEndPlay
  (params (EndPlayReason :type EEndPlayReason%20Enum :default "Destroyed"))
  (bind _playeractions (Variables|Default|GetPlayerActions))
  (bind _grid (Variables|/Game/Blueprints/Player/BP_PlayerActions.BP_PlayerActions_C|GetGrid _playeractions))
  (|CallParentFunction EndPlayReason)
  (Default|ClearStatefromTiles _grid "NewEnumerator3")
  (Default|ClearStatefromTiles _grid "NewEnumerator4"))

(fn ConstructionScript
  (|CallParentFunction))

(fn FindReachableTiles
  (params (Unit :type BP%20Unit%20Object%20Reference))
  (if (!= Unit (Variables|Default|GetCurrentUnitForReachables))
    (bind _output_get (Variables|Default|SetCurrentUnitForReachables Unit))
    (Default|ClearStatefromTiles (Variables|/Game/Blueprints/Player/BP_PlayerActions.BP_PlayerActions_C|GetGrid (Variables|Default|GetPlayerActions)) "NewEnumerator4")
    (EventDispatchers|BindEventtoOnPathfindingCompleted (Variables|/Game/Blueprints/Grid/BP_Grid.BP_Grid_C|GetGridPathfinding_Reachable (Variables|/Game/Blueprints/Player/BP_PlayerActions.BP_PlayerActions_C|GetGrid (Variables|Default|GetPlayerActions))) (EventDispatchers|CreateEvent :!event OnPathfindingCompleteReachables))
    (Default|FindPath (Variables|/Game/Blueprints/Grid/BP_Grid.BP_Grid_C|GetGridPathfinding_Reachable (Variables|/Game/Blueprints/Player/BP_PlayerActions.BP_PlayerActions_C|GetGrid (Variables|Default|GetPlayerActions))) (Variables|/Game/Blueprints/Units/BP_Unit.BP_Unit_C|GetCurrentGridIndex _output_get) (Utilities|Struct|MakeIntPoint -999 -999) (.CanWalkDiagonally (Utilities|Struct|BreakS_UnitData_Stats (.Stats (Utilities|Struct|BreakS_UnitData (Variables|/Game/Blueprints/Units/BP_Unit.BP_Unit_C|GetUnitData (Variables|Default|GetCurrentUnitForReachables)))))) (.ValidTileTypes (Utilities|Struct|BreakS_UnitData_Stats (.Stats (Utilities|Struct|BreakS_UnitData (Variables|/Game/Blueprints/Units/BP_Unit.BP_Unit_C|GetUnitData (Variables|Default|GetCurrentUnitForReachables)))))) 0.0 0.0 true (.MoveDistance (Utilities|Struct|BreakS_UnitData_Stats (.Stats (Utilities|Struct|BreakS_UnitData (Variables|/Game/Blueprints/Units/BP_Unit.BP_Unit_C|GetUnitData (Variables|Default|GetCurrentUnitForReachables)))))))))

(fn OnPathfindingCompleteReachables
  (params (Reachable%20Tiles :type Array%20of%20Int%20Point%20Structures))
  (if (not (Variables|Default|GetIsUnitMoving))
    (for _array_element Reachable%20Tiles
      (Default|AddTileStatetoTile (Variables|/Game/Blueprints/Player/BP_PlayerActions.BP_PlayerActions_C|GetGrid (Variables|Default|GetPlayerActions)) _array_element "NewEnumerator4"))))

(fn BindEventsfromUnit
  (params (Unit :type BP%20Unit%20Object%20Reference))
  (EventDispatchers|BindEventtoOnStartMoving Unit (EventDispatchers|CreateEvent :!event OnUnitStartMoving))
  (EventDispatchers|BindEventtoOnUnitReachedDestination Unit (EventDispatchers|CreateEvent :!event OnUnitFinishedMoving)))

(fn OnUnitStartMoving
  (params (Unit :type BP%20Unit%20Object%20Reference))
  (bind _playeractions (Variables|Default|GetPlayerActions))
  (bind _grid (Variables|/Game/Blueprints/Player/BP_PlayerActions.BP_PlayerActions_C|GetGrid _playeractions))
  (Default|ClearStatefromTiles _grid "NewEnumerator4")
  (Default|ClearStatefromTiles _grid "NewEnumerator3")
  (Default|UpdateSelectedTilesandUnits _playeractions (Variables|/Game/Blueprints/Units/BP_Unit.BP_Unit_C|GetCurrentGridIndex Unit) false true)
  (Variables|Default|SetCurrentUnitForReachables 0)
  (Variables|Default|SetIsUnitMoving true))

(fn UnbindEventsfromUnits
  (params (Unit :type BP%20Unit%20Object%20Reference))
  (EventDispatchers|UnbindEventfromOnStartMoving Unit (EventDispatchers|CreateEvent :!event OnUnitStartMoving))
  (EventDispatchers|UnbindEventfromOnUnitReachedDestination Unit (EventDispatchers|CreateEvent :!event OnUnitFinishedMoving)))

(fn ExecuteHoveredAction
  (params (Index :type Int%20Point%20Structure))
  (bind _playeractions (Variables|Default|GetPlayerActions))
  (bind _hoveredunit (Variables|/Game/Blueprints/Player/BP_PlayerActions.BP_PlayerActions_C|GetHoveredUnit _playeractions))
  (|CallParentFunction Index)
  (if (not (Variables|Default|GetIsUnitMoving))
    (Utilities|IsValid _hoveredunit
      (:Is%20Valid
        (CallFunction|FindReachableTiles _hoveredunit)
        (CallFunction|GeneratePath))
      (:Is%20Not%20Valid
        (if (> (Utilities|Array|Length (Variables|/Game/Blueprints/Player/BP_PlayerActions.BP_PlayerActions_C|GetSelectedUnits _playeractions)) 0)
          (CallFunction|FindReachableTiles (Utilities|Array|Get(acopy) (Variables|/Game/Blueprints/Player/BP_PlayerActions.BP_PlayerActions_C|GetSelectedUnits (Variables|Default|GetPlayerActions))))
          (CallFunction|GeneratePath))))))

(fn GeneratePath
  (bind _playeractions (Variables|Default|GetPlayerActions))
  (bind _selectedunits (Variables|/Game/Blueprints/Player/BP_PlayerActions.BP_PlayerActions_C|GetSelectedUnits _playeractions))
  (bind _output (Utilities|Array|Get(acopy) _selectedunits))
  (bind _unitdata (Variables|/Game/Blueprints/Units/BP_Unit.BP_Unit_C|GetUnitData _output))
  (bind _stats (Utilities|Struct|BreakS_UnitData _unitdata))
  (bind (_validtiletypes _canwalkdiagonally _movedistance) (Utilities|Struct|BreakS_UnitData_Stats _stats))
  (Default|ClearStatefromTiles (Variables|/Game/Blueprints/Player/BP_PlayerActions.BP_PlayerActions_C|GetGrid (Variables|Default|GetPlayerActions)) "NewEnumerator3")
  (Utilities|Array|Clear (Variables|Default|GetPath))
  (if (Default|HasSelectedUnits (Variables|Default|GetPlayerActions))
    (if (.CanMove (Utilities|Struct|BreakS_UnitData_Stats (.Stats (Utilities|Struct|BreakS_UnitData (Variables|/Game/Blueprints/Units/BP_Unit.BP_Unit_C|GetUnitData _output)))))
      (Default|FindPath (Variables|/Game/Blueprints/Grid/BP_Grid.BP_Grid_C|GetGrid%20Pathfinding (Variables|/Game/Blueprints/Player/BP_PlayerActions.BP_PlayerActions_C|GetGrid (Variables|Default|GetPlayerActions))) (Variables|/Game/Blueprints/Units/BP_Unit.BP_Unit_C|GetCurrentGridIndex _output) (Variables|/Game/Blueprints/Player/BP_PlayerActions.BP_PlayerActions_C|GetHoveredTile (Variables|Default|GetPlayerActions)) _canwalkdiagonally _validtiletypes 0.0 0.0 false _movedistance))))

(fn OnPathFindingCompletedPath
  (params (Path :type Array%20of%20Int%20Point%20Structures))
  (bind _output_get (Variables|Default|SetPath Path))
  (for _array_element _output_get
    (Default|AddTileStatetoTile (Variables|/Game/Blueprints/Player/BP_PlayerActions.BP_PlayerActions_C|GetGrid (Variables|Default|GetPlayerActions)) _array_element "NewEnumerator3")))

(fn ExecuteAction
  (params (Index :type Int%20Point%20Structure))
  (bind _playeractions (Variables|Default|GetPlayerActions))
  (bind _selectedunits (Variables|/Game/Blueprints/Player/BP_PlayerActions.BP_PlayerActions_C|GetSelectedUnits _playeractions))
  (bind _output (Utilities|Array|Get(acopy) _selectedunits))
  (|CallParentFunction Index)
  (if (and (> (Utilities|Array|Length (Variables|Default|GetPath)) 0) (Default|HasSelectedUnits (Variables|Default|GetPlayerActions)))
    (CallFunction|BindEventsfromUnit _output)
    (Default|MoveUnit (Variables|/Game/Blueprints/Player/BP_PlayerActions.BP_PlayerActions_C|GetCombatManager (Variables|Default|GetPlayerActions)) _output (Variables|Default|GetPath))
    (Utilities|Array|Clear (Variables|Default|GetPath))))

(fn OnUnitFinishedMoving
  (params (Unit :type BP%20Unit%20Object%20Reference) (Index :type Int%20Point%20Structure))
  (bind _playeractions (Variables|Default|GetPlayerActions))
  (CallFunction|ExecuteHoveredAction (Variables|/Game/Blueprints/Player/BP_PlayerActions.BP_PlayerActions_C|GetHoveredTile (Variables|Default|GetPlayerActions)))
  (CallFunction|UnbindEventsfromUnits Unit)
  (Variables|Default|SetIsUnitMoving false)
  (Default|SetCanMove Unit false)
  (Default|ClearAllSelections _playeractions)
  (if (Default|CanMoveorAct Unit)
    (Default|UpdateSelectedTilesandUnits _playeractions Index true false)))