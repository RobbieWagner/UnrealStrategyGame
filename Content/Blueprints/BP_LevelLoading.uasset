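; BP_LevelLoading is a Blueprint that switches between streaming levels, keeping the active one in a Level variable.
; On BeginPlay it force-loads that stored level.
; LoadLevel acts when the requested level differs or Force is set, unloading and hiding the previous streaming level, then storing the new one and flagging it loaded and visible.
; Streaming levels are looked up by converting Level to a name, with validity checks before changes.
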(event EventBeginPlay
  (CallFunction|LoadLevel (Variables|Default|GetLevel) true))

(fn ConstructionScript)

(fn LoadLevel
  (params (Level :type String) (Force :type Boolean))
  (if (or (Utilities|Enum|NotEqual(Enum) Level (Variables|Default|GetLevel)) Force)
    (Utilities|FlowControl|Sequence
      (:then_0
        (if (Utilities|IsValid (Class|GameplayStatics|GetStreamingLevel (Utilities|String|StringToName (Variables|Default|GetLevel))))
          (Variables|/Script/Engine.LevelStreaming|SetbShouldBeLoaded (Class|GameplayStatics|GetStreamingLevel (Utilities|String|StringToName (Variables|Default|GetLevel))) false)
          (Variables|/Script/Engine.LevelStreaming|SetbShouldBeVisible (Class|GameplayStatics|GetStreamingLevel (Utilities|String|StringToName (Variables|Default|GetLevel))) false)))
      (:then_1
        (bind _output_get (Variables|Default|SetLevel Level))
        (if (Utilities|IsValid (Class|GameplayStatics|GetStreamingLevel (Utilities|String|StringToName _output_get)))
          (Variables|/Script/Engine.LevelStreaming|SetbShouldBeLoaded (Class|GameplayStatics|GetStreamingLevel (Utilities|String|StringToName _output_get)) true)
          (Variables|/Script/Engine.LevelStreaming|SetbShouldBeVisible (Class|GameplayStatics|GetStreamingLevel (Utilities|String|StringToName _output_get)) true))))))