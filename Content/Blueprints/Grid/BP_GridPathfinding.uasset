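; Grid pathfinding Blueprint that runs an A*-style search between two square-grid tiles, filtering neighbours by tile type and height step.
; FindPath runs instantly or time-sliced through a delay and per-frame millisecond budget, broadcasting data updates and completion.
; AnalyzeNextTile expands the open list's first tile, and GeneratePath walks parent links back from the target.
; InsertIntoTilesFound's constant-true branch bypasses cost-sorted insertion, so tiles append in discovery order.
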(event Custom|FindPathWithDelay
  (Utilities|FlowControl|Sequence
    (:then_0
      (Variables|Default|SetLoopStartTime (Math|DateTime|Now) :!label _label)
      (if (> (Utilities|Array|Length (Variables|Default|GetTilesFound)) 0)
        (bind _found_target (CallFunction|AnalyzeNextTile))
        (if _found_target :!label _label_2
          (bind _path (CallFunction|GeneratePath))
          (Default|CallOnPathfindingCompleted _path)
          (else
            (if (> (Variables|Default|GetMaxMSPerFrame) 0.0)
              (if (< (Class|KismetMathLibrary|GetTotalMilliseconds (- (Math|DateTime|Now) (Variables|Default|GetLoopStartTime))) (Variables|Default|GetMaxMSPerFrame))
                (goto _label_2)
                (else
                  _)))
            (Utilities|FlowControl|RetriggerableDelay (Variables|Default|GetPathfindingDelay))
            (Utilities|FlowControl|Gate true :!label _label_3
              (:Exit
                (goto _label)))))
        (else
          (Default|CallOnPathfindingCompleted (Utilities|Array|MakeArray)))))
    (:then_1
      (goto _label_3 Open))))

(event Custom|CloseDelayGate
  (Utilities|FlowControl|Gate true) ; enters at Close
)

(event EventBeginPlay)

(event Collision|EventActorBeginOverlap
  (params (OtherActor :type Actor%20Object%20Reference)))

(event EventTick
  (params (DeltaSeconds :type Float%20%28single-precision%29)))

(fn ConstructionScript)

(fn GetValidTileNeighbors
  (params (Index :type Int%20Point%20Structure) (IncludeDiagonals :type Boolean) (ValidTileTypes :type Array%20of%20E_TileType%20Enums :default "NewEnumerator0"))
  (Variables|Default|SetInputTile (.Value (Utilities|Map|Find (Variables|/Game/Blueprints/Grid/BP_Grid.BP_Grid_C|GetGridTiles (Variables|Default|GetGrid)) Index)))
  (bind _neighbors (CallFunction|GetNeighborIndexes Index IncludeDiagonals))
  (for _array_element _neighbors
    (Variables|Default|SetAdjacentTile (.Value (Utilities|Map|Find (Variables|/Game/Blueprints/Grid/BP_Grid.BP_Grid_C|GetGridTiles (Variables|Default|GetGrid)) _array_element)))
    (if (Utilities|Array|ContainsItem ValidTileTypes (.tiletype (Variables|Default|GetAdjacentTile)))
      (if (<= (Math|Float|Absolute(Float) (- (.z (.location (.transform (Variables|Default|GetAdjacentTile)))) (.z (.location (.transform (Variables|Default|GetInputTile)))))) (* (.z (Default|GetTileScale (Variables|Default|GetGrid))) 1e+02))
        (Utilities|Array|Add (LocalVariables|Getret) (Utilities|Struct|MakeS_PathfindingData (.index (Variables|Default|GetAdjacentTile)) (Utilities|Select :Index (.tiletype (Variables|Default|GetAdjacentTile)) :NewEnumerator0 0 :NewEnumerator1 1 :NewEnumerator2 0 :NewEnumerator3 2 :NewEnumerator4 1) 999999 999999 Index)))))
  (return (LocalVariables|Getret)))

(fn GetSquareGridNeighborsIndexes
  (params (Index :type Int%20Point%20Structure) (IncludeDiagonals :type Boolean))
  (bind _intpoint (Utilities|Struct|MakeIntPoint -1 0))
  (bind _intpoint_2 (Utilities|Struct|MakeIntPoint 1 0))
  (bind _intpoint_3 (Utilities|Struct|MakeIntPoint 0 1))
  (bind _intpoint_4 (Utilities|Struct|MakeIntPoint 0 -1))
  (bind _returnvalue (+ Index _intpoint))
  (bind _returnvalue_2 (+ Index _intpoint_2))
  (bind _returnvalue_3 (+ Index _intpoint_3))
  (bind _returnvalue_4 (+ Index _intpoint_4))
  (bind _array (Utilities|Array|MakeArray _returnvalue _returnvalue_2 _returnvalue_3 _returnvalue_4))
  (if IncludeDiagonals
    (bind _output_get (Variables|Default|SetreturnArray _array))
    (Utilities|Array|AppendArray _output_get (Utilities|Array|MakeArray (+ Index (Utilities|Struct|MakeIntPoint -1 -1)) (+ Index (Utilities|Struct|MakeIntPoint 1 -1)) (+ Index (Utilities|Struct|MakeIntPoint -1 1)) (+ Index (Utilities|Struct|MakeIntPoint 1 1))))
    (return (Variables|Default|GetreturnArray))
    (else
      (return _array))))

(fn GetNeighborIndexes
  (params (Index :type Int%20Point%20Structure) (IncludeDiagonals :type Boolean))
  (switch Utilities|FlowControl|Switch|SwitchonE_GridShape (Variables|/Game/Blueprints/Grid/BP_Grid.BP_Grid_C|GetTile%20Shape (Variables|Default|GetGrid))
    (:NewEnumerator0
      (return (CallFunction|GetSquareGridNeighborsIndexes Index IncludeDiagonals)))))

(fn FindPath
  (params (Start :type Int%20Point%20Structure) (Target :type Int%20Point%20Structure) (UseDiagonals :type Boolean) (Valid%20Tile%20Types :type Array%20of%20E_TileType%20Enums :default "NewEnumerator0") (Delay :type Float%20%28double-precision%29) (MaxMS :type Float%20%28double-precision%29))
  (bind _array (Utilities|Array|MakeArray))
  (CallFunction|ClearPathfindingData)
  (Variables|Default|SetStart Start)
  (Variables|Default|SetTarget Target)
  (Variables|Default|SetUse%20Diagonals UseDiagonals)
  (Variables|Default|SetValid%20Tile%20Types Valid%20Tile%20Types)
  (Variables|Default|SetPathfindingDelay Delay)
  (Variables|Default|SetMaxMSPerFrame MaxMS)
  (CallFunction|CloseDelayGate)
  (bind _isvalid (CallFunction|IsInputDataValid))
  (if _isvalid
    (CallFunction|AddTiletoPathFinder (Utilities|Struct|MakeS_PathfindingData (Variables|Default|GetStart) 1 0 (CallFunction|GetCostBetweenTiles (Variables|Default|GetStart) (Variables|Default|GetTarget) (Variables|Default|GetUse%20Diagonals)) "(X=-999,Y=-999)"))
    (if (> (Variables|Default|GetPathfindingDelay) 0.0)
      (CallFunction|FindPathwithDelay)
      (return (Utilities|Array|MakeArray))
      (else
        (while (> (Utilities|Array|Length (Variables|Default|GetTilesFound)) 0)
          (bind _found_target (CallFunction|AnalyzeNextTile))
          (if _found_target
            (bind _path (CallFunction|GeneratePath))
            (Default|CallOnPathfindingCompleted _path)
            (return _path)))
        (Default|CallOnPathfindingCompleted _array)
        (return _array)))
    (else
      (Default|CallOnPathfindingCompleted (Utilities|Array|MakeArray)))))

(fn IsInputDataValid
  (if (!= (Variables|Default|GetStart) (Variables|Default|GetTarget))
    (if (Default|IsTileWalkable (Variables|Default|GetGrid) (Variables|Default|GetStart))
      (if (Default|IsTileWalkable (Variables|Default|GetGrid) (Variables|Default|GetTarget))
        (if (Utilities|Array|ContainsItem (Variables|Default|GetValid%20Tile%20Types) (.tiletype (Utilities|Struct|BreakS_TileData (.Value (Utilities|Map|Find (Variables|/Game/Blueprints/Grid/BP_Grid.BP_Grid_C|GetGridTiles (Variables|Default|GetGrid)) (Variables|Default|GetTarget))))))
          (return true)
          (else
            (return false)))
        (else
          (return false)))
      (else
        (return false)))
    (else
      (return false))))

(fn AddTiletoPathFinder
  (params (PathfindingData :type S%20Pathfinding%20Data%20Structure))
  (bind _index (Utilities|Struct|BreakS_PathfindingData PathfindingData))
  (Utilities|Map|Add (Variables|Default|GetPathfindingData) _index PathfindingData)
  (CallFunction|InsertIntoTilesFound PathfindingData)
  (Default|CallOnPathfindingDataUpdated _index))

(fn GetCostBetweenTiles
  (params (Tile%201 :type Int%20Point%20Structure) (Tile%202 :type Int%20Point%20Structure) (UseDiagonals :type Boolean))
  (bind _returnvalue (- Tile%201 Tile%202))
  (bind _returnvalue_2 (- Tile%201 Tile%202))
  (if UseDiagonals
    (return (Math|Integer|Max(Integer) (Math|Integer|Absolute(Integer) (.x _returnvalue_2)) (Math|Integer|Absolute(Integer) (.y _returnvalue_2))))
    (else
      (return (+ (Math|Integer|Absolute(Integer) (.x _returnvalue)) (Math|Integer|Absolute(Integer) (.y _returnvalue)))))))

(fn AnalyzeNextTile
  (bind _pathfindingdata (CallFunction|PullCheapestTilefromList))
  (bind _output_get (Variables|Default|SetCurrentTile _pathfindingdata))
  (Default|CallOnPathfindingDataUpdated (.Index (Utilities|Struct|BreakS_PathfindingData _output_get)))
  (bind _pathdata (CallFunction|GetValidTileNeighbors (.Index (Utilities|Struct|BreakS_PathfindingData (Variables|Default|GetCurrentTile))) (Variables|Default|GetUse%20Diagonals) (Variables|Default|GetValid%20Tile%20Types)))
  (Variables|Default|SetCurrentNeighbors _pathdata)
  (while (> (Utilities|Array|Length (Variables|Default|GetCurrentNeighbors)) 0)
    (bind _istarget (CallFunction|DiscoverNextNeighbor))
    (if _istarget
      (return true)))
  (return false))

(fn GeneratePath
  (LocalVariables|SetCurrent (Variables|Default|GetTarget))
  (while (!= (LocalVariables|GetCurrent) (Variables|Default|GetStart))
    (Utilities|Array|Add (LocalVariables|GetInvertedPath) (LocalVariables|GetCurrent))
    (LocalVariables|SetCurrent (.LastIndex (Utilities|Struct|BreakS_PathfindingData (.Value (Utilities|Map|Find (Variables|Default|GetPathfindingData) (LocalVariables|GetCurrent)))))))
  (bind _arrayelement (Utilities|Array|ReverseforEachLoop (LocalVariables|GetInvertedPath))
    (:LoopBody
      (Utilities|Array|Add (LocalVariables|Getret) _arrayelement))
    (:Completed
      (return (LocalVariables|Getret)))))

(fn PullCheapestTilefromList
  (LocalVariables|SetTileIndex (Utilities|Array|Get(acopy) (Variables|Default|GetTilesFound)))
  (Utilities|Array|RemoveIndex (Variables|Default|GetTileSortingCosts))
  (Utilities|Array|RemoveIndex (Variables|Default|GetTilesFound))
  (Utilities|Array|Add (Variables|Default|GetAnalyzedTiles) (LocalVariables|GetTileIndex))
  (return (.Value (Utilities|Map|Find (Variables|Default|GetPathfindingData) (LocalVariables|GetTileIndex)))))

(fn DiscoverNextNeighbor
  (Variables|Default|SetCurrentNeighbor (Utilities|Array|Get(acopy) (Variables|Default|GetCurrentNeighbors)))
  (Utilities|Array|RemoveIndex (Variables|Default|GetCurrentNeighbors))
  (if (not (Utilities|Array|ContainsItem (Variables|Default|GetAnalyzedTiles) (.Index (Utilities|Struct|BreakS_PathfindingData (Variables|Default|GetCurrentNeighbor)))))
    (LocalVariables|SetCostFromStart (+ (.Cost (Utilities|Struct|BreakS_PathfindingData (Variables|Default|GetCurrentTile))) (.Cost (Utilities|Struct|BreakS_PathfindingData (Variables|Default|GetCurrentNeighbor)))))
    (bind _output_get (LocalVariables|SetIndexInTiles (Utilities|Array|FindItem (Variables|Default|GetTilesFound) (.Index (Utilities|Struct|BreakS_PathfindingData (Variables|Default|GetCurrentNeighbor))))))
    (if (== _output_get -1)
      _
      (else
        (bind _output_get_2 (Variables|Default|SetCurrentNeighbor (.Value (Utilities|Map|Find (Variables|Default|GetPathfindingData) (.Index (Utilities|Struct|BreakS_PathfindingData (Variables|Default|GetCurrentNeighbor)))))))
        (if (< (LocalVariables|GetCostFromStart) (.Cost (Utilities|Struct|BreakS_PathfindingData _output_get_2)))
          (Utilities|Array|RemoveIndex (Variables|Default|GetTilesFound) (LocalVariables|GetIndexInTiles))
          (Utilities|Array|RemoveIndex (Variables|Default|GetTileSortingCosts) (LocalVariables|GetIndexInTiles))
          (else
            (return false)))))
    (CallFunction|AddTiletoPathFinder (Utilities|Struct|MakeS_PathfindingData (.Index (Utilities|Struct|BreakS_PathfindingData (Variables|Default|GetCurrentNeighbor))) (.Cost (Utilities|Struct|BreakS_PathfindingData (Variables|Default|GetCurrentNeighbor))) (LocalVariables|GetCostFromStart) (CallFunction|GetCostBetweenTiles (.Index (Utilities|Struct|BreakS_PathfindingData (Variables|Default|GetCurrentNeighbor))) (Variables|Default|GetTarget) (Variables|Default|GetUse%20Diagonals)) (.Index (Utilities|Struct|BreakS_PathfindingData (Variables|Default|GetCurrentTile)))))
    (if (Class|KismetMathLibrary|EqualIntPointIntPoint (.Index (Utilities|Struct|BreakS_PathfindingData (Variables|Default|GetCurrentNeighbor))) (Variables|Default|GetTarget))
      (return true)
      (else
        (return false)))
    (else
      (return false))))

(fn InsertIntoTilesFound
  (params (TileData :type S%20Pathfinding%20Data%20Structure))
  (bind _tilesortingcosts (Variables|Default|GetTileSortingCosts))
  (LocalVariables|SetSortingCost (CallFunction|GetTileSortingCost TileData))
  (if true
    (Utilities|Array|Add (Variables|Default|GetTileSortingCosts) (LocalVariables|GetSortingCost) :!label _label)
    (Utilities|Array|Add (Variables|Default|GetTilesFound) (.Index (Utilities|Struct|BreakS_PathfindingData TileData)))
    (elif (>= (LocalVariables|GetSortingCost) (Utilities|Array|Get(acopy) _tilesortingcosts (Utilities|Array|LastIndex _tilesortingcosts)))
      (goto _label)
      (else
        (bind (_array_element _array_index) (Utilities|Array|ForEachLoopwithBreak (Variables|Default|GetTileSortingCosts) :!label _label_2)
          (:LoopBody
            (if (>= _array_element (LocalVariables|GetSortingCost))
              (Utilities|Array|Insert (Variables|Default|GetTileSortingCosts) (LocalVariables|GetSortingCost) _array_index)
              (Utilities|Array|Insert (Variables|Default|GetTilesFound) (.Index (Utilities|Struct|BreakS_PathfindingData TileData)) _array_index)
              (goto _label_2 Break))))))))

(fn ClearPathfindingData
  (Utilities|Map|Clear (Variables|Default|GetPathfindingData))
  (Utilities|Array|Clear (Variables|Default|GetTileSortingCosts))
  (Utilities|Array|Clear (Variables|Default|GetTilesFound))
  (Utilities|Array|Clear (Variables|Default|GetAnalyzedTiles))
  (Default|CallOnPathfindingDataCleared))

(fn IsDiagonal
  (params (Index%201 :type Int%20Point%20Structure) (Index%202 :type Int%20Point%20Structure))
  (bind _neighbors (CallFunction|GetNeighborIndexes Index%201 false))
  (return (not (Utilities|Array|ContainsItem _neighbors Index%202))))

(fn GetTileSortingCost
  (params (PatfindingData :type S%20Pathfinding%20Data%20Structure%20%28by%20ref%29))
  (bind (_index _cost _costfromstart _costtotarget _lastindex) (Utilities|Struct|BreakS_PathfindingData PatfindingData))
  (return (+ (CallFunction|IsDiagonal _index _lastindex) (* (+ _costfromstart _costtotarget) 2))))