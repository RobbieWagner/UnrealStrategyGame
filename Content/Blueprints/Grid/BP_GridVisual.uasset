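; Grid visual actor that renders a grid's tiles through two child instanced-mesh actors, one standard and one tactical.
; Tile updates refresh walkable tiles on the offset standard mesh and pass data to the tactical layer, which colors by tile type.
; Tactical tiles stretch in Z by height above the lowest tile, forming columns.
; Tactical mode hides "NotTactical" actors and lazily rebuilds that layer via a dirty flag checked inside that actor loop.
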(event EventBeginPlay
  (Actor|Tick|SetActorTickEnabled false))

(event Collision|EventActorBeginOverlap
  (params (OtherActor :type Actor%20Object%20Reference)))

(event EventTick
  (params (DeltaSeconds :type Float%20%28single-precision%29)))

(fn ConstructionScript)

(fn InitializeGridVisual
  (params (Grid :type BP%20Grid%20Object%20Reference))
  (Variables|Default|SetGrid Grid)
  (Variables|Default|SetGrid%20Mesh%20Inst (.AsBP%20Grid%20Mesh%20Inst (Utilities|Casting|CastToBP_GridMeshInst (Variables|/Script/Engine.ChildActorComponent|GetChildActor (Variables|Default|GetChildActor_GridMeshInst)))))
  (Variables|Default|SetGridMeshInst_Tactical (.AsBP%20Grid%20Mesh%20Inst (Utilities|Casting|CastToBP_GridMeshInst (Variables|/Script/Engine.ChildActorComponent|GetChildActor (Variables|Default|GetChildActor_GridMeshInst_Tactical)))))
  (Default|InitializeGridMeshInst (Variables|Default|GetGrid%20Mesh%20Inst) (.FlatMesh (Utilities|Struct|BreakS_GridShapeData (Default|GetGridShapeData (Variables|Default|GetGrid)))) (.FlatMaterial (Utilities|Struct|BreakS_GridShapeData (Default|GetGridShapeData (Variables|Default|GetGrid)))) false "QueryOnly")
  (Default|InitializeGridMeshInst (Variables|Default|GetGridMeshInst_Tactical) (.FlatMesh (Utilities|Struct|BreakS_GridShapeData (Default|GetGridShapeData (Variables|Default|GetGrid)))) (.FlatMaterial (Utilities|Struct|BreakS_GridShapeData (Default|GetGridShapeData (Variables|Default|GetGrid)))) true "QueryOnly")
  (Transformation|SetActorLocation "0, 0, 0" false false)
  (CallFunction|SetGroundOffset (Variables|Default|GetOffsetFromGround))
  (CallFunction|SetGridLowestZ 9999.0))

(fn SetGroundOffset
  (params (Offset :type Float%20%28double-precision%29))
  (bind _output_get (Variables|Default|SetOffsetFromGround Offset))
  (Transformation|SetRelativeLocation (Variables|Default|GetChildActor_GridMeshInst) (Math|Vector|MakeVector 0.0 0.0 _output_get) false false))

(fn DestroyGridVisual
  (bind _grid_mesh_inst (Variables|Default|GetGrid%20Mesh%20Inst))
  (bind _gridmeshinst_tactical (Variables|Default|GetGridMeshInst_Tactical))
  (Utilities|FlowControl|Sequence
    (:then_0
      (Utilities|IsValid _grid_mesh_inst
        (:Is%20Valid
          (Default|ClearInstances _grid_mesh_inst))))
    (:then_1
      (Utilities|IsValid _gridmeshinst_tactical
        (:Is%20Valid
          (Default|ClearInstances _gridmeshinst_tactical))))
    (:then_2
      (CallFunction|SetGridLowestZ 9999.0))))

(fn UpdateTileVisual
  (params (Tile%20Data :type S%20Tile%20Data%20Structure))
  (Utilities|FlowControl|Sequence
    (:then_0
      (Default|RemoveInstance (Variables|Default|GetGrid%20Mesh%20Inst) (.index Tile%20Data))
      (if (CallFunction|IsTileWalkable (.tiletype Tile%20Data))
        (Default|AddInstance (Variables|Default|GetGrid%20Mesh%20Inst) (.index Tile%20Data) (.transform Tile%20Data) (.currentstates Tile%20Data) (.tiletype Tile%20Data))))
    (:then_1
      (CallFunction|UpdateTileVisualTactical Tile%20Data))))

(fn UpdateTileVisualTactical
  (params (Data :type S%20Tile%20Data%20Structure))
  (bind _grid (Variables|Default|GetGrid))
  (bind _location (Math|Transform|BreakTransform (.transform Data)))
  (bind (_location_2 _rotation _scale) (Math|Transform|BreakTransform (.transform Data)))
  (bind _returnvalue (Default|GetGridShapeData _grid))
  (bind _meshsize (Utilities|Struct|BreakS_GridShapeData _returnvalue))
  (bind _z (Math|Vector|BreakVector _meshsize))
  (Utilities|FlowControl|Sequence
    (:then_0
      (if (< (.z _location) (Variables|Default|GetGridLowestZ))
        (CallFunction|SetGridLowestZ (.z _location))))
    (:then_1
      (if (Variables|Default|GetIs%20Tactical)
        (Default|RemoveInstance (Variables|Default|GetGridMeshInst_Tactical) (.index Data))
        (if (Utilities|Enum|NotEqual(Enum) (.tiletype Data) "NewEnumerator0")
          (Default|AddInstance (Variables|Default|GetGridMeshInst_Tactical) (.index Data) (Math|Transform|MakeTransform _location_2 _rotation (Math|Vector|MakeVector (.x _scale) (.y _scale) (/ (+ (- (.Z (Math|Vector|BreakVector (.Location (Math|Transform|BreakTransform (.transform Data))))) (Variables|Default|GetGridLowestZ)) _z) _z))) (.currentstates Data) (.tiletype Data)))
        (else
          (Variables|Default|SetGenerateTacticalOnEnable true))))))

(fn SetGridLowestZ
  (params (GridLowestZ :type Float%20%28double-precision%29))
  (Variables|Default|SetGridLowestZ GridLowestZ)
  (Variables|Default|SetGenerateTacticalOnEnable true))

(fn SetIsTactical
  (params (IsTactical :type Boolean))
  (bind _output_get (Variables|Default|SetIs%20Tactical IsTactical))
  (Development|SetHiddeninGame (Variables|Default|GetChildActor_GridMeshInst_Tactical) (not _output_get) false)
  (bind _outactors (Actor|GetAllActorswithTag "NotTactical"))
  (for _array_element _outactors
    (Rendering|SetActorHiddenInGame _array_element (Variables|Default|GetIs%20Tactical))
    (if (and (Variables|Default|GetIs%20Tactical) (Variables|Default|GetGenerateTacticalOnEnable))
      (Variables|Default|SetGenerateTacticalOnEnable false)
      (bind _values (Utilities|Map|Values (Variables|/Game/Blueprints/Grid/BP_Grid.BP_Grid_C|GetGridTiles (Variables|Default|GetGrid))))
      (for _array_element_2 _values
        (CallFunction|UpdateTileVisualTactical _array_element_2)))))