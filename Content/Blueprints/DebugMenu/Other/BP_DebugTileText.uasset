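; Debug actor that draws tile indexes and pathfinding data as floating text over BP_Grid tiles.
; SetDebugTileText toggles entrance cost, target and start costs, sort order and index display, then refreshes or clears the text.
; It spawns one TextRenderActor per tile on demand, cached by index and destroyed when that tile has nothing to show.
; It binds to grid and pathfinding events, with a retriggerable delay available to batch full refreshes.
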(event Custom|UpdateDebugTextAfterDelay
  (params (Index :type Int%20Point%20Structure))
  (Utilities|FlowControl|RetriggerableDelay 0.1)
  (CallFunction|UpdateTextonAllTiles))

(event EventBeginPlay
  (bind _returnvalue (Actor|GetActorOfClass "/Game/Blueprints/Grid/BP_Grid.BP_Grid_C"))
  (bind _output_get (Variables|Default|SetGrid _returnvalue))
  (EventDispatchers|BindEventtoOnGridDestroyed _output_get (EventDispatchers|CreateEvent :!event DestroyAllTextActors))
  (EventDispatchers|BindEventtoOnTileDataUpdated _output_get (EventDispatchers|CreateEvent :!event UpdateDebugTileText))
  (EventDispatchers|BindEventtoOnPathfindingDataCleared (Variables|/Game/Blueprints/Grid/BP_Grid.BP_Grid_C|GetGrid%20Pathfinding (Variables|Default|GetGrid)) (EventDispatchers|CreateEvent :!event UpdateTextonAllTiles))
  (EventDispatchers|BindEventtoOnPathfindingDataUpdated (Variables|/Game/Blueprints/Grid/BP_Grid.BP_Grid_C|GetGrid%20Pathfinding (Variables|Default|GetGrid)) (EventDispatchers|CreateEvent :!event Custom|UpdateDebugTextAfterDelay)))

(event Collision|EventActorBeginOverlap
  (params (OtherActor :type Actor%20Object%20Reference)))

(event EventTick
  (params (DeltaSeconds :type Float%20%28single-precision%29)))

(fn ConstructionScript)

(fn GetTextActor
  (params (Index :type Int%20Point%20Structure))
  (bind _output_get (LocalVariables|SetActor (.Value (Utilities|Map|Find (Variables|Default|GetSpawnedTextActors) Index))))
  (Utilities|IsValid _output_get
    (:Is%20Valid
      (return _output_get))
    (:Is%20Not%20Valid
      (bind _returnvalue (Game|SpawnActorfromClass "/Script/Engine.TextRenderActor" (Math|Transform|MakeTransform "0, 0, 0" "0, 0, 0" "1.000000,1.000000,1.000000") "AlwaysSpawn" "MultiplyWithRoot" 0 0))
      (bind _output_get_2 (LocalVariables|SetActor _returnvalue))
      (Utilities|Map|Add (Variables|Default|GetSpawnedTextActors) Index _output_get_2)
      (Actor|Tick|SetActorTickEnabled (LocalVariables|GetActor))
      (Collision|SetActorEnableCollision (LocalVariables|GetActor) false)
      (Rendering|Components|TextRender|SetHorizontalAlignment (Variables|/Script/Engine.TextRenderActor|GetTextRender (LocalVariables|GetActor)) "EHTA_Center")
      (Class|TextRenderComponent|SetVerticalAlignment (Variables|/Script/Engine.TextRenderActor|GetTextRender (LocalVariables|GetActor)) "EVRTA_TextCenter")
      (return (LocalVariables|GetActor)))))

(fn DestroyTextActor
  (params (Index :type Int%20Point%20Structure))
  (bind _output_get (LocalVariables|SetActor (.Value (Utilities|Map|Find (Variables|Default|GetSpawnedTextActors) Index))))
  (Utilities|IsValid _output_get
    (:Is%20Valid
      (Actor|DestroyActor _output_get)
      (Utilities|Map|Remove (Variables|Default|GetSpawnedTextActors) Index))))

(fn DestroyAllTextActors
  (bind _values (Utilities|Map|Values (Variables|Default|GetSpawnedTextActors)))
  (for _array_element _values
    (Actor|DestroyActor _array_element))
  (Utilities|Map|Clear (Variables|Default|GetSpawnedTextActors)))

(fn UpdateDebugTileText
  (params (Index :type Int%20Point%20Structure))
  (bind _grid (Variables|Default|GetGrid))
  (bind _grid_2 (Variables|Default|GetGrid))
  (bind _gridtiles (Variables|/Game/Blueprints/Grid/BP_Grid.BP_Grid_C|GetGridTiles _grid))
  (bind _grid_pathfinding (Variables|/Game/Blueprints/Grid/BP_Grid.BP_Grid_C|GetGrid%20Pathfinding _grid_2))
  (bind (_value _returnvalue) (Utilities|Map|Find _gridtiles Index))
  (bind _tilesfound (Variables|/Game/Blueprints/Grid/BP_GridPathfinding.BP_GridPathfinding_C|GetTilesFound _grid_pathfinding))
  (bind _returnvalue_2 (Utilities|Array|FindItem _tilesfound Index))
  (if (CallFunction|DisplayAnyText)
    (if _returnvalue
      (LocalVariables|SetData _value)
      (Utilities|FlowControl|Sequence
        (:then_0
          (Utilities|FlowControl|Sequence
            (:then_0
              (if (Variables|Default|GetShowIndexes)
                (Utilities|Array|Add (LocalVariables|GetText) (Utilities|String|Append (Utilities|String|ToString(Integer) (.x Index)) ", " (Utilities|String|ToString(Integer) (.y Index))))))
            (:then_1
              (if (Math|Boolean|ORBoolean (Variables|Default|GetShowTileEntranceCost) (Variables|Default|GetShowCostToTarget) (Variables|Default|GetShowCostFromStart) (Variables|Default|GetShowSortOrder))
                (if (.ReturnValue (Utilities|Map|Find (Variables|/Game/Blueprints/Grid/BP_GridPathfinding.BP_GridPathfinding_C|GetPathfindingData (Variables|/Game/Blueprints/Grid/BP_Grid.BP_Grid_C|GetGrid%20Pathfinding (Variables|Default|GetGrid))) Index))
                  (LocalVariables|SetPathfindingData (.Value (Utilities|Map|Find (Variables|/Game/Blueprints/Grid/BP_GridPathfinding.BP_GridPathfinding_C|GetPathfindingData (Variables|/Game/Blueprints/Grid/BP_Grid.BP_Grid_C|GetGrid%20Pathfinding (Variables|Default|GetGrid))) Index)))
                  (Utilities|FlowControl|Sequence
                    (:then_0
                      (if (Variables|Default|GetShowTileEntranceCost)
                        (Utilities|Array|Add (LocalVariables|GetText) (Utilities|String|Append "C: " (Utilities|String|ToString(Integer) (.Cost (Utilities|Struct|BreakS_PathfindingData (LocalVariables|GetPathfindingData))))))))
                    (:then_1
                      (if (Variables|Default|GetShowCostToTarget)
                        (if (!= (.CostToTarget (Utilities|Struct|BreakS_PathfindingData (LocalVariables|GetPathfindingData))) 99999)
                          (Utilities|Array|Add (LocalVariables|GetText) (Utilities|String|Append "T: " (Utilities|String|ToString(Integer) (.CostToTarget (Utilities|Struct|BreakS_PathfindingData (LocalVariables|GetPathfindingData)))))))))
                    (:then_2
                      (if (Variables|Default|GetShowCostFromStart)
                        (if (!= (.CostFromStart (Utilities|Struct|BreakS_PathfindingData (LocalVariables|GetPathfindingData))) 99999)
                          (Utilities|Array|Add (LocalVariables|GetText) (Utilities|String|Append "S: " (Utilities|String|ToString(Integer) (.CostFromStart (Utilities|Struct|BreakS_PathfindingData (LocalVariables|GetPathfindingData)))))))))
                    (:then_3
                      (if (Variables|Default|GetShowSortOrder)
                        (if (!= _returnvalue_2 -1)
                          (Utilities|Array|Add (LocalVariables|GetText) (Utilities|String|Append "O: " (Utilities|String|ToString(Integer) _returnvalue_2) "(" (Utilities|String|ToString(Integer) (Utilities|Array|Get(acopy) (Variables|/Game/Blueprints/Grid/BP_GridPathfinding.BP_GridPathfinding_C|GetTileSortingCosts _grid_pathfinding) _returnvalue_2)) ")")))))))))))
        (:then_1
          (if (> (Utilities|Array|Length (LocalVariables|GetText)) 0)
            (bind _textrenderactor (CallFunction|GetTextActor Index))
            (LocalVariables|SetActor _textrenderactor)
            (Rendering|Components|TextRender|SetText (Variables|/Script/Engine.TextRenderActor|GetTextRender (LocalVariables|GetActor)) (Utilities|Text|ToText(String) (Utilities|String|JoinStringArray (LocalVariables|GetText) " 
")))
            (Transformation|SetActorTransform (LocalVariables|GetActor) (Math|Transform|MakeTransform (+ (.location (.transform (LocalVariables|GetData))) "0.000000,0.000000,4.000000") "90.000000,180.000000,0.000000" "2.000000,2.000000,2.000000"))
            (else
              (CallFunction|DestroyTextActor Index)))))
      (else
        (CallFunction|DestroyTextActor Index)))))

(fn SetDebugTileText
  (params (ShowIndexes :type Boolean) (ShowEntranceCost :type Boolean) (ShowCostToTarget :type Boolean) (ShowCostFromStart :type Boolean) (ShowSortOrder :type Boolean))
  (Variables|Default|SetShowIndexes ShowIndexes)
  (Variables|Default|SetShowTileEntranceCost ShowEntranceCost)
  (Variables|Default|SetShowCostToTarget ShowCostToTarget)
  (Variables|Default|SetShowCostFromStart ShowCostFromStart)
  (Variables|Default|SetShowSortOrder ShowSortOrder)
  (CallFunction|DisplayDebugTileText))

(fn DisplayDebugTileText
  (if (CallFunction|DisplayAnyText)
    (bind _keys (Utilities|Map|Keys (Variables|/Game/Blueprints/Grid/BP_Grid.BP_Grid_C|GetGridTiles (Variables|Default|GetGrid))))
    (for _array_element _keys
      (CallFunction|UpdateDebugTileText _array_element))
    (else
      (CallFunction|DestroyAllTextActors))))

(fn DisplayAnyText
  (return (Math|Boolean|ORBoolean (Variables|Default|GetShowIndexes) (Variables|Default|GetShowTileEntranceCost) (Variables|Default|GetShowCostToTarget) (Variables|Default|GetShowCostFromStart) (Variables|Default|GetShowSortOrder))))

(fn UpdateTextonAllTiles
  (bind _keys (Utilities|Map|Keys (Variables|/Game/Blueprints/Grid/BP_Grid.BP_Grid_C|GetGridTiles (Variables|Default|GetGrid))))
  (for _array_element _keys
    (CallFunction|UpdateDebugTileText _array_element)))