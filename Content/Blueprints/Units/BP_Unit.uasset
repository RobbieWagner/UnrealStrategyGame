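; Grid-based unit actor with a Paper2D flipbook sprite, configured from a data row chosen by UnitType.
; Path following moves it tile by tile on a Timeline scaled to TileTransitionTime, firing dispatchers at start, each tile and destination.
; Grid index deltas choose directional animations from the unit data's flipbook map, with debug prints on change.
; A set of unit states drives the sprite material, with the first match in enum order taking priority.
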(event Custom|Event_FollowPath
  (params (Path :type Array%20of%20Int%20Point%20Structures))
  (bind _timeline_moveunit (Variables|Default|GetTimeline_MoveUnit))
  (Default|CallOnStartMoving self)
  (if (> (Utilities|Array|Length Path) 0)
    (Variables|Default|SetCurrentPath Path)
    (Variables|Default|SetPosition (Transformation|GetActorLocation))
    (Variables|Default|SetDestination (.Location (Math|Transform|BreakTransform (.transform (Utilities|Struct|BreakS_TileData (.Value (Utilities|Map|Find (Variables|/Game/Blueprints/Grid/BP_Grid.BP_Grid_C|GetGridTiles (Variables|Default|GetGrid)) (Utilities|Array|Get(acopy) (Variables|Default|GetCurrentPath)))))))))
    (Components|Timeline|SetPlayRate _timeline_moveunit (/ (Components|Timeline|GetTimelineLength _timeline_moveunit) (Variables|Default|GetTileTransitionTime)))
    (bind _locationalpha (Timeline|Timeline_MoveUnit PlayFromStart)
      (:Update
        (Transformation|SetActorLocation (Math|Vector|Lerp(Vector) (Variables|Default|GetPosition) (Variables|Default|GetDestination) _locationalpha) false false)
        (CallFunction|SetAnimationStateBasedonMovementDirection (- (Utilities|Array|Get(acopy) (Variables|Default|GetCurrentPath)) (Variables|Default|GetCurrentGridIndex))))
      (:Finished
        (Default|CallOnUnitReachedNewTile self (Utilities|Array|Get(acopy) (Variables|Default|GetCurrentPath)))
        (Utilities|Array|RemoveIndex (Variables|Default|GetCurrentPath))
        (CallFunction|EventContinueFollowPath)))))

(event Custom|Event_ContinueFollowPath
  (bind _timeline_moveunit (Variables|Default|GetTimeline_MoveUnit))
  (if (> (Utilities|Array|Length (Variables|Default|GetCurrentPath)) 0)
    (Variables|Default|SetPosition (Transformation|GetActorLocation))
    (Variables|Default|SetDestination (.Location (Math|Transform|BreakTransform (.transform (Utilities|Struct|BreakS_TileData (.Value (Utilities|Map|Find (Variables|/Game/Blueprints/Grid/BP_Grid.BP_Grid_C|GetGridTiles (Variables|Default|GetGrid)) (Utilities|Array|Get(acopy) (Variables|Default|GetCurrentPath)))))))))
    (Components|Timeline|SetPlayRate _timeline_moveunit (/ (Components|Timeline|GetTimelineLength _timeline_moveunit) (Variables|Default|GetTileTransitionTime)))
    (bind _locationalpha (Timeline|Timeline_MoveUnit PlayFromStart)
      (:Update
        (Transformation|SetActorLocation (Math|Vector|Lerp(Vector) (Variables|Default|GetPosition) (Variables|Default|GetDestination) _locationalpha) false false)
        (CallFunction|SetAnimationStateBasedonMovementDirection (- (Utilities|Array|Get(acopy) (Variables|Default|GetCurrentPath)) (Variables|Default|GetCurrentGridIndex))))
      (:Finished
        (Default|CallOnUnitReachedNewTile self (Utilities|Array|Get(acopy) (Variables|Default|GetCurrentPath)))
        (Utilities|Array|RemoveIndex (Variables|Default|GetCurrentPath))
        (CallFunction|EventContinueFollowPath)))
    (else
      (CallFunction|SetAnimationState "NewEnumerator0")
      (Default|CallOnUnitReachedDestination self (Variables|Default|GetCurrentGridIndex)))))

(event EventBeginPlay
  (CallFunction|SetAnimationState "NewEnumerator0"))

(fn ConstructionScript
  (bind _unitdata (CallFunction|GetUnitDataRowbyType (Variables|Default|GetUnitType)))
  (CallFunction|SetUnitData _unitdata))

(fn UpdateUnitVisual
  (Rendering|Material|SetMaterial (Variables|Default|GetFlipbook) 0 (Utilities|Select :Index (CallFunction|GetMostImportantUnitState) :NewEnumerator1 "/Game/Art/Units/SpriteGlow_LightBlue.SpriteGlow_LightBlue" :NewEnumerator2 "/Game/Art/Units/SpriteGlow_White.SpriteGlow_White" :NewEnumerator4 "/Game/Art/Units/LitSprite_Damaged.LitSprite_Damaged" :NewEnumerator3 "/Game/Art/Units/LitSprite_Burning.LitSprite_Burning" :NewEnumerator0 "/Game/Art/Units/DefaultLitSpriteMaterial.DefaultLitSpriteMaterial")))

(fn AddStatetoUnit
  (params (State :type E_UnitState%20Enum :default "NewEnumerator0"))
  (Utilities|Array|AddUnique (Variables|Default|GetUnitStates) State)
  (CallFunction|UpdateUnitVisual))

(fn RemoveStatefromUnit
  (params (State :type E_UnitState%20Enum :default "NewEnumerator0"))
  (bind _returnvalue (Utilities|Array|RemoveItem (Variables|Default|GetUnitStates) State))
  (CallFunction|UpdateUnitVisual)
  (return _returnvalue))

(fn GetMostImportantUnitState
  (bind _enumvalue (|ForEachE_UnitState)
    (:LoopBody
      (if (Utilities|Array|ContainsItem (Variables|Default|GetUnitStates) _enumvalue)
        (return _enumvalue)))))

(fn SetFlipbookMaterial
  (params (Material :type Material%20Object%20Reference))
  (for _index (range 0 (- (Class|PaperFlipbookComponent|GetFlipbookLengthinFrames (Variables|Default|GetFlipbook)) 1))
    (Rendering|Material|SetMaterial (Variables|Default|GetFlipbook) _index (Utilities|Select :Index (CallFunction|GetMostImportantUnitState) :NewEnumerator1 "/Game/Art/Units/SpriteGlow_LightBlue.SpriteGlow_LightBlue" :NewEnumerator2 "/Game/Art/Units/SpriteGlow_White.SpriteGlow_White" :NewEnumerator4 "/Game/Art/Units/LitSprite_Damaged.LitSprite_Damaged" :NewEnumerator3 "/Game/Art/Units/LitSprite_Burning.LitSprite_Burning" :NewEnumerator0 "/Game/Art/Units/DefaultLitSpriteMaterial.DefaultLitSpriteMaterial"))))

(fn SetUnitData
  (params (Data :type S%20Unit%20Data%20Structure))
  (Variables|Default|SetUnitData Data)
  (CallFunction|SetAnimationState "NewEnumerator0")
  (Physics|SetEnableGravity (Variables|Default|GetFlipbook) false)
  (CallFunction|UpdateUnitVisual))

(fn CanbeMovedbyPlayer
  (return true))

(fn SetAnimationStateBasedonMovementDirection
  (params (delta :type Int%20Point%20Structure))
  (bind (_x _y) (Utilities|Struct|BreakIntPoint delta))
  (Utilities|FlowControl|Sequence
    (:then_0
      (LocalVariables|SetdeltaX _x)
      (LocalVariables|SetdeltaY _y))
    (:then_1
      (if (> (Math|Integer|Absolute(Integer) (LocalVariables|GetdeltaY)) (Math|Integer|Absolute(Integer) (LocalVariables|GetdeltaX)))
        (if (> (LocalVariables|GetdeltaY) 0)
          (bind _changedsuccessfully (CallFunction|SetAnimationState "NewEnumerator5"))
          (if _changedsuccessfully
            (Development|PrintString "B"))
          (elif (< (LocalVariables|GetdeltaY) 0)
            (bind _changedsuccessfully_2 (CallFunction|SetAnimationState "NewEnumerator4"))
            (if _changedsuccessfully_2
              (Development|PrintString "U"))
            (else
              (bind _changedsuccessfully_3 (CallFunction|SetAnimationState "NewEnumerator0"))
              (if _changedsuccessfully_3
                (Development|PrintString "I1")))))
        (elif (> (LocalVariables|GetdeltaX) 0)
          (bind _changedsuccessfully_4 (CallFunction|SetAnimationState "NewEnumerator3"))
          (if _changedsuccessfully_4
            (Development|PrintString "R"))
          (elif (< (LocalVariables|GetdeltaX) 0)
            (bind _changedsuccessfully_5 (CallFunction|SetAnimationState "NewEnumerator2"))
            (if _changedsuccessfully_5
              (Development|PrintString "L"))
            (else
              (bind _changedsuccessfully_6 (CallFunction|SetAnimationState "NewEnumerator0"))
              (if _changedsuccessfully_6
                (Development|PrintString "I2")))))))))

(fn SetGrid
  (params (newGrid :type BP%20Grid%20Object%20Reference))
  (Variables|Default|SetGrid newGrid))

(fn SetAnimationState
  (params (State :type E_UnitAnimationState%20Enum :default "NewEnumerator7"))
  (bind _unitdata (Variables|Default|GetUnitData))
  (bind (_value _returnvalue) (Utilities|Map|Find (.animationstates _unitdata) State))
  (if _returnvalue
    (bind _output_get (LocalVariables|SetnewFlipbook _value))
    (if (!= _output_get (Variables|Default|GetCurrentFlipBook))
      (bind _output_get_2 (Variables|Default|SetCurrentFlipBook _value))
      (bind _returnvalue_2 (Sprite|SetFlipbook (Variables|Default|GetFlipbook) _output_get_2))
      (return _returnvalue_2)
      (else
        (return false)))
    (else
      (return false))))