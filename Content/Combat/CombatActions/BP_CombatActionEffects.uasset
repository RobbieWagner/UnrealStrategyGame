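; Short-lived combat actor that presents an action's effects on the grid, then destroys itself.
; On BeginPlay it spawns a BP_PlayActionFlipbook for each flipbook entry at every affected index, plus one BP_DisplayActionUI at the origin index.
; Completion events are bound on the spawned actors; a finished-animation counter and a UI-done flag gate destruction until both flipbooks and UI finish.
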(event Custom|PlayEffects
  (CallFunction|PlayFlipbooks)
  (CallFunction|DisplayActionUI))

(event EventBeginPlay
  (CallFunction|PlayEffects))

(fn ConstructionScript)

(fn PlayFlipbooks
  (Variables|Default|SetAnimationComplete 0)
  (Variables|Default|SetAnimationsUntilDeath (Utilities|Array|Length (Variables|Default|GetFlipbookData)))
  (for _array_element (Variables|Default|GetFlipbookData)
    (for _array_element_2 (Variables|Default|GetEffectedIndexes)
      (CallFunction|SpawnFlipbook _array_element_2 _array_element)
      (Math|Integer|IncrementInt (Variables|Default|GetAnimationsUntilDeath)))
    (Math|Integer|DecrementInt (Variables|Default|GetAnimationsUntilDeath))))

(fn IncrementCompletedAnimations
  (Math|Integer|IncrementInt (Variables|Default|GetAnimationComplete)
    (:%20%20
      (CallFunction|CheckforDeath))))

(fn CheckforDeath
  (if (and (== (Variables|Default|GetAnimationsUntilDeath) (Variables|Default|GetAnimationComplete)) (Variables|Default|GetisUIDone))
    (Actor|DestroyActor)))

(fn SpawnFlipbook
  (params (Index :type Int%20Point%20Structure) (S_CombatAction_FlipbookData :type S%20Combat%20Action%20Flipbook%20Data%20Structure%20%28by%20ref%29))
  (bind (_flipbook _sourcelocation _material) (Utilities|Struct|BreakS_CombatAction_FlipbookData S_CombatAction_FlipbookData))
  (bind _returnvalue (Game|SpawnActorfromClass "/Game/Combat/EffectComponents/BP_PlayActionFlipbook.BP_PlayActionFlipbook_C" (Math|Transform|MakeTransform (+ (Default|GetLocationbyIndex (Variables|Default|GetGrid) Index) "0.000000,5.000000,0.000000")) "AlwaysSpawn" "MultiplyWithRoot" 0 _flipbook _material (Variables|Default|GetGrid) (Variables|Default|GetTargetIndex) 0))
  (EventDispatchers|BindEventtoOnEffectComplete _returnvalue (EventDispatchers|CreateEvent :!event IncrementCompletedAnimations)))

(fn DisplayActionUI
  (bind _returnvalue (Game|SpawnActorfromClass "/Game/Combat/EffectComponents/BP_DisplayActionUI.BP_DisplayActionUI_C" (Math|Transform|MakeTransform (Default|GetLocationbyIndex (Variables|Default|GetGrid) (Variables|Default|GetOriginIndex))) "Undefined" "MultiplyWithRoot" 0 (Variables|Default|GetGrid) (Variables|Default|GetTargetIndex) 0))
  (EventDispatchers|BindEventtoOnEffectComplete _returnvalue (EventDispatchers|CreateEvent :!event CompleteUIDisplay)))

(fn CompleteUIDisplay
  (Variables|Default|SetisUIDone true)
  (CallFunction|CheckforDeath))