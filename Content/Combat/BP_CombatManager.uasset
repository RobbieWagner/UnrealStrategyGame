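; Combat manager that tracks units on the tile grid and executes combat actions against them.
; Keeps tile occupancy and unit positions synced as units move or tiles change, destroying units on invalid tile types.
; Actions resolve user or target tiles, optionally as AoE, then spawn effects and afflict living units with one shared HP roll.
; Ranges exclude unwalkable tiles and, if required, those where any of four offset line traces is blocked.
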(event EventBeginPlay
  (bind _grid (Variables|Default|GetGrid))
  (EventDispatchers|BindEventtoOnGridGenerated _grid (EventDispatchers|CreateEvent :!event OnGridGenerated))
  (EventDispatchers|BindEventtoOnTileDataUpdated _grid (EventDispatchers|CreateEvent :!event OnTileDataUpdated)))

(fn ConstructionScript)

(fn AddUnittoGrid
  (params (Unit :type BP%20Unit%20Object%20Reference) (Index :type Int%20Point%20Structure))
  (Utilities|Array|Add (Variables|Default|GetCombatUnits) Unit)
  (CallFunction|SetUnitIndexonGrid Unit Index false)
  (Default|SetGrid Unit (Variables|Default|GetGrid))
  (EventDispatchers|BindEventtoOnUnitReachedNewTile Unit (EventDispatchers|CreateEvent :!event OnUnitReachedNewTile)))

(fn RemoveUnitfromGrid
  (params (Unit :type BP%20Unit%20Object%20Reference) (Destroy :type Boolean))
  (Utilities|Array|RemoveItem (Variables|Default|GetCombatUnits) Unit)
  (CallFunction|SetUnitIndexonGrid Unit (Utilities|Struct|MakeIntPoint -999 -999) false)
  (if Destroy
    (Actor|DestroyActor Unit)))

(fn SetUnitIndexonGrid
  (params (Unit :type BP%20Unit%20Object%20Reference) (Index :type Int%20Point%20Structure) (Force :type Boolean))
  (bind _grid (Variables|Default|GetGrid))
  (bind _gridtiles (Variables|/Game/Blueprints/Grid/BP_Grid.BP_Grid_C|GetGridTiles _grid))
  (bind (_value _returnvalue) (Utilities|Map|Find _gridtiles Index))
  (Utilities|FlowControl|Sequence
    (:then_0
      (if (or (!= (Variables|/Game/Blueprints/Units/BP_Unit.BP_Unit_C|GetCurrentGridIndex Unit) Index) Force)
        (Utilities|FlowControl|Sequence
          (:then_0
            (bind _output_get (LocalVariables|SetLastTile (.Value (Utilities|Map|Find (Variables|/Game/Blueprints/Grid/BP_Grid.BP_Grid_C|GetGridTiles (Variables|Default|GetGrid)) (Variables|/Game/Blueprints/Units/BP_Unit.BP_Unit_C|GetCurrentGridIndex Unit)))))
            (if (== (.UnitOnTile (Utilities|Struct|BreakS_TileData _output_get)) Unit)
              (bind _structout (Utilities|Struct|SetmembersinS_TileData (LocalVariables|GetLastTile) 0))
              (Utilities|Map|Add (Variables|/Game/Blueprints/Grid/BP_Grid.BP_Grid_C|GetGridTiles (Variables|Default|GetGrid)) (.index (Utilities|Struct|BreakS_TileData _structout)) _structout)))
          (:then_1
            (Variables|/Game/Blueprints/Units/BP_Unit.BP_Unit_C|SetCurrentGridIndex Unit Index)
            (if (!= Index (Utilities|Struct|MakeIntPoint -999 -999))
              (bind _structout_2 (Utilities|Struct|SetmembersinS_TileData (.Value (Utilities|Map|Find (Variables|/Game/Blueprints/Grid/BP_Grid.BP_Grid_C|GetGridTiles (Variables|Default|GetGrid)) Index)) Unit))
              (Utilities|Map|Add (Variables|/Game/Blueprints/Grid/BP_Grid.BP_Grid_C|GetGridTiles (Variables|Default|GetGrid)) (.index (Utilities|Struct|BreakS_TileData _structout_2)) _structout_2))))))
    (:then_1
      (Transformation|SetActorLocation Unit (select _returnvalue (.Location (Math|Transform|BreakTransform (.transform (Utilities|Struct|BreakS_TileData _value)))) "-99999.000000,-99999.000000,-999990.000000") false false))))

(fn OnGridGenerated
  (bind _output_get (LocalVariables|SetCopyUnits (Variables|Default|GetCombatUnits)))
  (for _array_element _output_get
    (if (Utilities|Array|ContainsItem (.ValidTileTypes (Utilities|Struct|BreakS_UnitData_Stats (.Stats (Utilities|Struct|BreakS_UnitData (Variables|/Game/Blueprints/Units/BP_Unit.BP_Unit_C|GetUnitData _array_element))))) (.tiletype (Utilities|Struct|BreakS_TileData (.Value (Utilities|Map|Find (Variables|/Game/Blueprints/Grid/BP_Grid.BP_Grid_C|GetGridTiles (Variables|Default|GetGrid)) (Variables|/Game/Blueprints/Units/BP_Unit.BP_Unit_C|GetCurrentGridIndex _array_element))))))
      (CallFunction|SetUnitIndexonGrid :Unit _array_element :Force true)
      (else
        (CallFunction|RemoveUnitfromGrid _array_element true)))))

(fn OnTileDataUpdated
  (params (UpdatedTile :type Int%20Point%20Structure))
  (bind _output_get (LocalVariables|SetCopyUnits (Variables|Default|GetCombatUnits)))
  (bind _array_element (Utilities|Array|ForEachLoopwithBreak _output_get :!label _label)
    (:LoopBody
      (if (Class|KismetMathLibrary|EqualIntPointIntPoint UpdatedTile (Variables|/Game/Blueprints/Units/BP_Unit.BP_Unit_C|GetCurrentGridIndex _array_element))
        (if (Utilities|Array|ContainsItem (.ValidTileTypes (Utilities|Struct|BreakS_UnitData_Stats (.Stats (Utilities|Struct|BreakS_UnitData (Variables|/Game/Blueprints/Units/BP_Unit.BP_Unit_C|GetUnitData _array_element))))) (.tiletype (Utilities|Struct|BreakS_TileData (.Value (Utilities|Map|Find (Variables|/Game/Blueprints/Grid/BP_Grid.BP_Grid_C|GetGridTiles (Variables|Default|GetGrid)) (Variables|/Game/Blueprints/Units/BP_Unit.BP_Unit_C|GetCurrentGridIndex _array_element))))))
          (CallFunction|SetUnitIndexonGrid _array_element (Variables|/Game/Blueprints/Units/BP_Unit.BP_Unit_C|GetCurrentGridIndex _array_element) false)
          (goto _label Break)
          (else
            (CallFunction|RemoveUnitfromGrid _array_element true)
            (goto _label Break)))))))

(fn OnUnitReachedNewTile
  (params (Unit :type BP%20Unit%20Object%20Reference) (Index :type Int%20Point%20Structure))
  (CallFunction|SetUnitIndexonGrid Unit Index false))

(fn ExecuteCombatAction
  (params (Action :type E_CombatAction%20Enum :default "NewEnumerator0") (Origin%20Index :type Int%20Point%20Structure) (Target%20Index :type Int%20Point%20Structure))
  (bind _grid (Variables|Default|GetGrid))
  (bind _gridtiles (Variables|/Game/Blueprints/Grid/BP_Grid.BP_Grid_C|GetGridTiles _grid))
  (bind _value (Utilities|Map|Find _gridtiles Origin%20Index))
  (bind _unitontile (Utilities|Struct|BreakS_TileData _value))
  (bind _data (CallFunction|GetDatafromCombatAction Action))
  (bind _output_get (LocalVariables|SetCombatActionData _data))
  (switch Utilities|FlowControl|Switch|SwitchonE_CombatAction_SourceLocation (.SourceLocation (Utilities|Struct|BreakS_CombatActionData _output_get))
    (:NewEnumerator1
      (if (Utilities|Enum|Equal(Enum) (.RangePattern (Utilities|Struct|BreakS_CombatAction_Execution (.AoE (Utilities|Struct|BreakS_CombatActionData (LocalVariables|GetCombatActionData))))) "NewEnumerator0")
        ;[0 0 0] User: Target is user
        (LocalVariables|SetActionExecutionTiles (Utilities|Array|MakeArray Origin%20Index))
        (else
          ;[0 0 0] AoE (User) Target is any tile in range originating from tje user's tile
          (LocalVariables|SetActionExecutionTiles (CallFunction|GetActionRange Origin%20Index (.AoE (Utilities|Struct|BreakS_CombatActionData (LocalVariables|GetCombatActionData)))))))
      (bind _returnvalue (Game|SpawnActorfromClass (.Effects (Utilities|Struct|BreakS_CombatAction_Assets (.Assets (Utilities|Struct|BreakS_CombatActionData (LocalVariables|GetCombatActionData))))) (Math|Transform|MakeTransform "0, 0, 0") "AlwaysSpawn" "MultiplyWithRoot" 0 (Variables|Default|GetGrid) Origin%20Index Target%20Index (LocalVariables|GetActionExecutionTiles) (.FlipbookData (Utilities|Struct|BreakS_CombatAction_Assets (.Assets (Utilities|Struct|BreakS_CombatActionData (LocalVariables|GetCombatActionData))))) 0 :!label _label))
      (LocalVariables|SetActionEffects _returnvalue)
      (Default|CallOnActionExecuted)
      (Utilities|FlowControl|Sequence
        (:then_0
          (Utilities|IsValid _unitontile
            (:Is%20Valid
              (Default|UnitUseAction _unitontile Target%20Index))))
        (:then_1
          (LocalVariables|SetActionStatsReal (Utilities|Struct|MakeS_CombatAction_Stats_Real (CallFunction|MinMaxRandom (.HPModifier (Utilities|Struct|BreakS_CombatAction_Stats (.Stats (Utilities|Struct|BreakS_CombatActionData (LocalVariables|GetCombatActionData)))))) (.Accuracy (Utilities|Struct|BreakS_CombatAction_Stats (.Stats (Utilities|Struct|BreakS_CombatActionData (LocalVariables|GetCombatActionData))))) (.TimeToImpact (Utilities|Struct|BreakS_CombatAction_Stats (.Stats (Utilities|Struct|BreakS_CombatActionData (LocalVariables|GetCombatActionData)))))))
          (for _array_element (LocalVariables|GetActionExecutionTiles)
            (Utilities|IsValid (.UnitOnTile (Utilities|Struct|BreakS_TileData (.Value (Utilities|Map|Find (Variables|/Game/Blueprints/Grid/BP_Grid.BP_Grid_C|GetGridTiles (Variables|Default|GetGrid)) _array_element))))
              (:Is%20Valid
                (bind _output_get_2 (LocalVariables|SetUnit (.UnitOnTile (Utilities|Struct|BreakS_TileData (.Value (Utilities|Map|Find (Variables|/Game/Blueprints/Grid/BP_Grid.BP_Grid_C|GetGridTiles (Variables|Default|GetGrid)) _array_element))))))
                (if (!= (.CurrentHealth (Utilities|Struct|BreakS_UnitData_Stats (.Stats (Utilities|Struct|BreakS_UnitData (Variables|/Game/Blueprints/Units/BP_Unit.BP_Unit_C|GetUnitData (LocalVariables|GetUnit)))))) 0)
                  (Default|UnitAfflictedbyAction _output_get_2 (LocalVariables|GetActionStatsReal) (LocalVariables|GetActionEffects)))))))))
    (:NewEnumerator2
      (if (Utilities|Enum|Equal(Enum) (.RangePattern (Utilities|Struct|BreakS_CombatAction_Execution (.AoE (Utilities|Struct|BreakS_CombatActionData (LocalVariables|GetCombatActionData))))) "NewEnumerator0")
        ;[0 0 0] Target: Target is selected tile in range
        (if (Utilities|Array|ContainsItem (CallFunction|GetActionRange Origin%20Index (.Execution (Utilities|Struct|BreakS_CombatActionData _output_get))) Target%20Index)
          (LocalVariables|SetActionExecutionTiles (Utilities|Array|MakeArray Target%20Index))
          (goto _label))
        (else
          ;[0 0 0] AoE (Target) Target is any tile in range originating from targeted tile
          (if (Utilities|Array|ContainsItem (CallFunction|GetActionRange Origin%20Index (.Execution (Utilities|Struct|BreakS_CombatActionData _output_get))) Target%20Index)
            (LocalVariables|SetActionExecutionTiles (CallFunction|GetActionRange Target%20Index (.AoE (Utilities|Struct|BreakS_CombatActionData (LocalVariables|GetCombatActionData)))))
            (goto _label)))))))

(fn GetActionRange
  (params (Origin :type Int%20Point%20Structure) (ExecutionData :type S%20Combat%20Action%20Execution%20Structure))
  (bind (_rangepattern _rangeminmax _requirelineofsight) (Utilities|Struct|BreakS_CombatAction_Execution ExecutionData))
  (bind _tilesinrange (CallFunction|GetTilesinActionRange Origin _rangepattern _rangeminmax))
  (bind _rangetiles (CallFunction|RemoveUnwalkableTiles _tilesinrange))
  (if _requirelineofsight
    (bind _rangetiles_2 (CallFunction|RemoveTilesOutOfSight Origin _rangetiles 75.0))
    (return _rangetiles_2)
    (else
      (return _rangetiles))))

(fn HasLineOfSight
  (params (OriginIndex :type Int%20Point%20Structure) (TargetIndex :type Int%20Point%20Structure) (Height :type Float%20%28double-precision%29))
  (bind _grid (Variables|Default|GetGrid))
  (bind _returnvalue (Math|Vector|MakeVector 0.0 0.0 Height))
  (bind _tilescale (Default|GetTileScale _grid))
  (bind _returnvalue_2 (/ _tilescale "4.000000,4.000000,4.000000"))
  (bind (_x _y) (Math|Vector|BreakVector _returnvalue_2))
  (LocalVariables|SetOriginTile (.Value (Utilities|Map|Find (Variables|/Game/Blueprints/Grid/BP_Grid.BP_Grid_C|GetGridTiles (Variables|Default|GetGrid)) OriginIndex)))
  (LocalVariables|SetTargetTile (.Value (Utilities|Map|Find (Variables|/Game/Blueprints/Grid/BP_Grid.BP_Grid_C|GetGridTiles (Variables|Default|GetGrid)) TargetIndex)))
  (LocalVariables|SetStart (+ (.Location (Math|Transform|BreakTransform (.transform (Utilities|Struct|BreakS_TileData (LocalVariables|GetOriginTile))))) _returnvalue))
  (LocalVariables|SetEnd (+ _returnvalue (.Location (Math|Transform|BreakTransform (.transform (Utilities|Struct|BreakS_TileData (LocalVariables|GetTargetTile)))))))
  (for _array_element (Utilities|Array|MakeArray (Math|Vector2D|MakeVector2D _x 0.0) (Math|Vector2D|MakeVector2D (* _x -1.0) 0.0) (Math|Vector2D|MakeVector2D 0.0 _y) (Math|Vector2D|MakeVector2D 0.0 (* _y -1.0)))
    (bind _returnvalue_3 (Collision|LineTraceByChannel (+ (LocalVariables|GetStart) _array_element) (LocalVariables|GetEnd) "TraceTypeQuery6" false 0 "None"))
    (if _returnvalue_3
      (return false)))
  (return true))

(fn RemoveTilesOutOfSight
  (params (Origin :type Int%20Point%20Structure) (Array :type Array%20of%20Int%20Point%20Structures) (UnitHeight :type Float%20%28double-precision%29))
  (for _array_element Array
    (if (CallFunction|HasLineOfSight Origin _array_element UnitHeight)
      (Utilities|Array|AddUnique (LocalVariables|Getret) _array_element)))
  (return (LocalVariables|Getret)))

(fn RemoveUnwalkableTiles
  (params (Array :type Array%20of%20Int%20Point%20Structures))
  (for _array_element Array
    (if (Default|IsTileWalkable (Variables|Default|GetGrid) _array_element)
      (Utilities|Array|AddUnique (LocalVariables|Getret) _array_element)))
  (return (LocalVariables|Getret)))