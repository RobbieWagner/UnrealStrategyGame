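; BP_PlayActionFlipbook is a combat effect component actor that plays a one-shot flipbook animation.
; On BeginPlay it applies the configured flipbook and material to its EffectAnimation component.
; It waits for the flipbook's length, fires the effect-complete call, then destroys itself.
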(event EventBeginPlay
  (bind _effectanimation (Variables|Default|GetEffectAnimation))
  (|CallParentFunction)
  (Sprite|SetFlipbook _effectanimation (Variables|Default|GetFlipbookAsset))
  (Rendering|Material|SetMaterial _effectanimation 0 (Variables|Default|GetMaterial))
  (Utilities|FlowControl|Delay (Class|PaperFlipbookComponent|GetFlipbookLength (Variables|Default|GetEffectAnimation)))
  (Default|CallOnEffectComplete)
  (Actor|DestroyActor))

(fn ConstructionScript
  (|CallParentFunction))