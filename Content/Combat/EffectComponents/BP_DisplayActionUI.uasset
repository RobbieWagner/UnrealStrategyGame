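; BP_DisplayActionUI is a combat effect actor that shows a brief animated icon at a target grid cell.
; On BeginPlay it moves to the grid location of TargetIndex and sets the DebugIdle1 texture on its W_image widget component.
; A timeline drives the widget's height, draw size and opacity.
; When the timeline finishes, it calls OnEffectComplete and destroys itself.
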(event EventBeginPlay
  (bind _imagewidget (Variables|Default|GetImageWidget))
  (|CallParentFunction)
  (Transformation|SetActorLocation (Default|GetLocationbyIndex (Variables|Default|GetGrid) (Variables|Default|GetTargetIndex)) false false)
  (bind _output_get (Variables|Default|SetW%20Image (.AsW%20Image (Utilities|Casting|CastToW_image (UserInterface|GetUserWidgetObject (Variables|Default|GetImageWidget))))))
  (Appearance|SetBrushfromTexture (Variables|/Game/Combat/EffectComponents/W_image.W_image_C|GetImage _output_get) "/Game/Art/Units/Debug/DebugIdle1.DebugIdle1" false)
  (bind (_direction _locationz _drawsize _opacity) (Timeline|UIAnimationTimeline PlayFromStart)
    (:Update
      (Transformation|SetRelativeLocation _imagewidget (Math|Vector|MakeVector 0.0 0.0 _locationz) false false)
      (Class|WidgetComponent|SetDrawSize _imagewidget (Math|Vector2D|MakeVector2D _drawsize _drawsize))
      (Widget|SetRenderOpacity (Variables|Default|GetW%20Image) _opacity))
    (:Finished
      (Default|CallOnEffectComplete)
      (Actor|DestroyActor))))

(fn ConstructionScript
  (|CallParentFunction))